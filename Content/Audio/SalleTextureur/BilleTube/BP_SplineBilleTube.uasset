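; Marble actor (bille) that travels along the spline of a referenced SplineChemin, likely inside a tube.
; The BougeObjet event plays a timeline at a rate of 1 / TempsPourFinir, so that variable controls the travel time.
; Each update maps timeline alpha to spline distance, setting location in world space and rotation from the spline's local space.
; The construction script applies the configurable ObjectMesh to the Sphere component.
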(event `Bouge Objet`
  (bind _spline (`/Game/Audio/SalleTextureur/BilleTube/BP_SplineBilleChemin.Spline` (`self.SplineChemin`)))
  ; La vitesse de la bille
  (`TimelineComponent.SetPlayRate` (`self.T_Bouge`) (/ 1.0 (`self.TempsPourFinir`)))
  (bind (_direction _bouge_) (`Timeline|T_Bouge`)
    (:`Update`
      (bind _returnvalue (`KismetMathLibrary.Lerp` 0.0 (`SplineComponent.GetSplineLength` _spline) _bouge_))
      ; objet qui bouge avec le spline
      (`self.K2_SetActorLocationAndRotation` (`SplineComponent.GetLocationAtDistanceAlongSpline` _spline _returnvalue "World") (`SplineComponent.GetRotationAtDistanceAlongSpline` _spline _returnvalue "Local")))))

(fn `UserConstructionScript`
  (`StaticMeshComponent.SetStaticMesh` (`self.Sphere`) (`self.Object mesh`)))