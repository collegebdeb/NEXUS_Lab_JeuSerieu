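; Level tool actor that starts a referenced Level Sequence when something overlaps its trigger box.
; On BeginPlay, if StartOnframe1 is valid, it plays and immediately pauses the sequence, apparently to hold it on its opening frame.
; The first overlap, with no filter on the overlapping actor, passes a DoOnce, destroys the trigger box and plays the sequence.
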(event `self.ReceiveBeginPlay`
  (bind _sequenceplayer (`LevelSequenceActor.SequencePlayer` (`self.LevelSequenceReference`)))
  ; Simple lvl sqc trigger code
  (`self.StartOnframe1`
    (:`then`
      (`MovieSceneSequencePlayer.Play` _sequenceplayer)
      (`MovieSceneSequencePlayer.Pause` _sequenceplayer))
    (:`else`)))

(event `self.TriggerBox.OnComponentBeginOverlap`
  (params (OverlappedComponent :type "PrimitiveComponent Object Reference") (OtherActor :type "Actor Object Reference") (OtherComp :type "PrimitiveComponent Object Reference") (OtherBodyIndex :type Integer) (bFromSweep :type Boolean) (SweepResult :type "HitResult Structure (by ref)"))
  ; Simple lvl sqc trigger code
  (`/Engine/EditorBlueprintResources/StandardMacros.DoOnce` false
    (:`Completed`
      (`ActorComponent.K2_DestroyComponent` (`self.TriggerBox`))
      (`MovieSceneSequencePlayer.Play` (`LevelSequenceActor.SequencePlayer` (`self.LevelSequenceReference`))))))

(fn `UserConstructionScript`)