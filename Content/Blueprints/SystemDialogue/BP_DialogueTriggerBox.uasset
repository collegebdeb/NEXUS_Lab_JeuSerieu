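; One-shot trigger box that plays a sequence of dialogue lines through the player pawn when overlapped.
; On first overlap it resets the pawn's message, then Speaking sends each line's text, speaker, portrait, sound and a self reference, unless the pawn is already speaking.
; A resettable DoOnce loops through the parallel arrays, timing each delay from text length, typing delay and skip time.
; After the last line it hides the message and destroys itself.
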(event `self.Box.OnComponentBeginOverlap`
  (params (OverlappedComponent :type "PrimitiveComponent Object Reference") (OtherActor :type "Actor Object Reference") (OtherComp :type "PrimitiveComponent Object Reference") (OtherBodyIndex :type Integer) (bFromSweep :type Boolean) (SweepResult :type "HitResult Structure (by ref)"))
  (bind _returnvalue (- (`self.CurrentDialogue`) 1))
  (bind _returnvalue_2 (+ (* (`|GetArrayItem` (`self.TextDelay`) _returnvalue) (`KismetStringLibrary.Len` (`|GetArrayItem` (`self.Dialogue`) _returnvalue))) (`|GetArrayItem` (`self.Time Until Skip`) _returnvalue)))
  (`/Engine/EditorBlueprintResources/StandardMacros.DoOnce` false
    (:`Completed`
      (set `self.CurrentDialogue` 0)
      (message `/Game/Blueprints/SystemDialogue/Interfaces/BPI_DialogueInfo.ResetDialogue` (`GameplayStatics.GetPlayerPawn` 0))
      (`KismetSystemLibrary.DelayUntilNextTick`)
      (`/Engine/EditorBlueprintResources/StandardMacros.DoOnce` false :!label _label
        (:`Completed`
          (`self.Speaking`)
          (if (>= (`self.CurrentDialogue`) (`KismetArrayLibrary.Array_Length` (`self.Dialogue`)))
            (`KismetSystemLibrary.Delay` _returnvalue_2)
            (message `/Game/Blueprints/SystemDialogue/Interfaces/BPI_DialogueInfo.HideDialogue` (`GameplayStatics.GetPlayerPawn` 0))
            (`self.K2_DestroyActor`)
            (else
              (`KismetSystemLibrary.Delay` _returnvalue_2)
              (`|ExecutionSequence`
                (:`then_0`
                  (goto _label :!via `Reset`))
                (:`then_1`
                  (goto _label))))))))))

(fn `Speaking`
  (bind _returnvalue (`GameplayStatics.GetPlayerPawn` 0))
  (bind _isspeaking_ (message `/Game/Blueprints/SystemDialogue/Interfaces/BPI_DialogueInfo.CheckSpeaking` _returnvalue))
  (if (not _isspeaking_)
    (message `/Game/Blueprints/SystemDialogue/Interfaces/BPI_DialogueInfo.Speaking` _returnvalue (`|GetArrayItem` (`self.Dialogue`) (`self.CurrentDialogue`)) (`|GetArrayItem` (`self.TextDelay`) (`self.CurrentDialogue`)) (`|GetArrayItem` (`self.Character Name`) (`self.CurrentDialogue`)) (`|GetArrayItem` (`self.CharacterImage`) (`self.CurrentDialogue`)) self (`|GetArrayItem` (`self.SoundToPlay`) (`self.CurrentDialogue`)))
    (bind _result (`/Engine/EditorBlueprintResources/StandardMacros.IncrementInt` (`self.CurrentDialogue`))
      (:`  `
        (`|ExecutionSequence`
          (:`then_0`
            (return))
          (:`then_1`
            (if (and (not _isspeaking_) (>= _result (`KismetArrayLibrary.Array_Length` (`self.Dialogue`))))
              (`self.K2_DestroyActor`))))))))

(fn `UserConstructionScript`)