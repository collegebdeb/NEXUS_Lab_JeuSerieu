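; A trigger box that plays a one-time sequence of dialogue lines from a data array when the player's hitbox enters it.
; Speaking sends the current entry to the player pawn unless a message is already showing, then advances the index.
; A reset-and-re-enter DoOnce loop times each line by text length, speed and skip delay.
; After the last line, it hides the dialogue and destroys itself.
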(event `self.Box.OnComponentBeginOverlap`
  (params (OverlappedComponent :type "PrimitiveComponent Object Reference") (OtherActor :type "Actor Object Reference") (OtherComp :type "PrimitiveComponent Object Reference") (OtherBodyIndex :type Integer) (bFromSweep :type Boolean) (SweepResult :type "HitResult Structure (by ref)"))
  (bind _dialoguedataasset (`self.DialogueDataAsset`))
  (bind _output (`|GetArrayItem` _dialoguedataasset (- (`self.CurrentDialogue`) 1)))
  (bind _returnvalue (+ (* (`/Game/Blueprints/SystemDialogue/PDA_LigneDialogue.TextSpeed` _output) (`KismetStringLibrary.Len` (`/Game/Blueprints/SystemDialogue/PDA_LigneDialogue.Dialogue` _output))) (`/Game/Blueprints/SystemDialogue/PDA_LigneDialogue.TimeBeforeSkip` _output)))
  (if (`ActorComponent.ComponentHasTag` OtherComp "PlayerHitBox")
    (`/Engine/EditorBlueprintResources/StandardMacros.DoOnce` false
      (:`Completed`
        (set `self.CurrentDialogue` 0)
        (message `/Game/Blueprints/SystemDialogue/Interfaces/BPI_DialogueInfo.ResetDialogue` (`GameplayStatics.GetPlayerPawn` 0))
        (`KismetSystemLibrary.DelayUntilNextTick`)
        (`/Engine/EditorBlueprintResources/StandardMacros.DoOnce` false :!label _label
          (:`Completed`
            (`self.Speaking`)
            (if (>= (`self.CurrentDialogue`) (`KismetArrayLibrary.Array_Length` _dialoguedataasset))
              (`KismetSystemLibrary.Delay` _returnvalue)
              (`KismetSystemLibrary.Delay` 2.0)
              (message `/Game/Blueprints/SystemDialogue/Interfaces/BPI_DialogueInfo.HideDialogue` (`GameplayStatics.GetPlayerPawn` 0))
              (`self.K2_DestroyActor`)
              (else
                (`KismetSystemLibrary.Delay` _returnvalue)
                (`|ExecutionSequence`
                  (:`then_0`
                    (goto _label :!via `Reset`))
                  (:`then_1`
                    (goto _label)))))))))))

(fn `Speaking`
  (bind _returnvalue (`GameplayStatics.GetPlayerPawn` 0))
  (bind _dialoguedataasset (`self.DialogueDataAsset`))
  (bind _isspeaking_ (message `/Game/Blueprints/SystemDialogue/Interfaces/BPI_DialogueInfo.CheckSpeaking` _returnvalue))
  (if (not _isspeaking_)
    (message `/Game/Blueprints/SystemDialogue/Interfaces/BPI_DialogueInfo.Speaking` _returnvalue (`|GetArrayItem` _dialoguedataasset (`self.CurrentDialogue`)) self)
    (bind _result (`/Engine/EditorBlueprintResources/StandardMacros.IncrementInt` (`self.CurrentDialogue`))
      (:`  `
        (`|ExecutionSequence`
          (:`then_0`
            (return))
          (:`then_1`
            (if (and (not _isspeaking_) (>= _result (`KismetArrayLibrary.Array_Length` _dialoguedataasset)))
              (`self.K2_DestroyActor`))))))))

(fn `UserConstructionScript`)