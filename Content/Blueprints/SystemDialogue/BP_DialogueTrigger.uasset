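; Trigger volume actor that plays a character dialogue once when the player pawn is inside it.
; Tick polls the overlap, so it also fires for a player already inside, and waits while the game mode flags another dialogue as running.
; When fired, it sets that flag and sends its Dialogues to the character's dialogue UI.
; An optional delay uses a timer that counts independently of overlap; the begin-overlap event has no effect.
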(event `self.ReceiveBeginPlay`
  ; Set Variables
  (set `self.Player` (`Controller.K2_GetPawn` (`GameplayStatics.GetPlayerController` 0)))
  (set `self.As GM First Person` (cast `/Game/FirstPerson/Blueprints/GM_FirstPerson` (`GameplayStatics.GetGameMode`) :!pure true)))

(event `self.ReceiveActorBeginOverlap`
  (params (OtherActor :type "Actor Object Reference"))
  ; TriggerEnter
  (cast `/Game/FirstPerson/Blueprints/BP_FirstPersonCharacter` OtherActor)
  (if (not (`/Game/FirstPerson/Blueprints/GM_FirstPerson.IsDialogueRunning` (`self.As GM First Person`)))
    _))

(event `self.ReceiveTick`
  (params (DeltaSeconds :type "Float (single-precision)"))
  (bind _isdelayedtrigger (`self.IsDelayedTrigger`))
  ; WhileTrigger (So it activates even when already in the triggerbox)
  (`|ExecutionSequence`
    (:`then_0`
      (if (and (not (`/Game/FirstPerson/Blueprints/GM_FirstPerson.IsDialogueRunning` (`self.As GM First Person`))) (`self.IsOverlappingActor` (`self.Player`)) (or (not _isdelayedtrigger) (and _isdelayedtrigger (>= (`self.TimeInTriggerBox`) (`self.TriggerDelay`)))))
        (`/Engine/EditorBlueprintResources/StandardMacros.DoOnce` false
          (:`Completed`
            (set `/Game/FirstPerson/Blueprints/GM_FirstPerson.IsDialogueRunning` true (`self.As GM First Person`)) ; So we don't have multiple dialogues interfering
            (message `/Game/Blueprints/SystemDialogue/Interfaces/BPI_DialogueData.RunDialogue` (`/Game/FirstPerson/Blueprints/BP_FirstPersonCharacter.UIDialogue` (cast `/Game/FirstPerson/Blueprints/BP_FirstPersonCharacter` (`self.Player`) :!pure true)) (`self.Dialogues`) true)))))
    (:`then_1`
      (`self.IsDelayedTrigger`
        (:`then`
          (set `self.TimeInTriggerBox` (+ (`self.TimeInTriggerBox`) DeltaSeconds)))
        (:`else`)))))

(fn `UserConstructionScript`)