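; Outdated dialogue component that holds lines of text with matching character names, images and text delays, indexed by a current dialogue counter.
; Its Speaking event only asks the player pawn whether a message is being spoken, and the branch on that result does nothing.
; The logic that calls SpeakingMessage on the pawn, advances the counter and wraps it to zero is disconnected, as are the array lookups.
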(event `Speaking`
  (bind _isspeaking_ (message `/Game/Blueprints/SystemDialogue/Interfaces/BPI_DialogueInfo.CheckSpeaking` (`GameplayStatics.GetPlayerPawn` 0)))
  (if _isspeaking_
    _))