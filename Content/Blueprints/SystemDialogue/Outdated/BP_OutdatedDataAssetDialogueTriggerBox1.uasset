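; Outdated one-shot trigger box that plays a sequence of dialogue lines when a component tagged PlayerHitBox overlaps it.
; Speaking sends each DialogueDataAsset entry to the player pawn when CheckSpeakingMessage is false.
; A re-entered DoOnce paces lines by text length, speed and skip time, then hides the message and destroys the actor.
; UpdateDialogue scans the line-asset folder via Asset Registry and copies TableDialogue rows into assets by Id.
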(event `self.Box.OnComponentBeginOverlap`
  (params (OverlappedComponent :type "PrimitiveComponent Object Reference") (OtherActor :type "Actor Object Reference") (OtherComp :type "PrimitiveComponent Object Reference") (OtherBodyIndex :type Integer) (bFromSweep :type Boolean) (SweepResult :type "HitResult Structure (by ref)"))
  (bind _dialoguedataasset (`self.DialogueDataAsset`))
  (bind _output (`|GetArrayItem` _dialoguedataasset (- (`self.CurrentDialogue`) 1)))
  (bind _returnvalue (+ (* (`/Game/Blueprints/SystemDialogue/Outdated/PDA_LigneDialogue.TextSpeed` _output) (`KismetStringLibrary.Len` (`/Game/Blueprints/SystemDialogue/Outdated/PDA_LigneDialogue.DialogueText` _output))) (`/Game/Blueprints/SystemDialogue/Outdated/PDA_LigneDialogue.TimeBeforeSkip` _output)))
  (if (`ActorComponent.ComponentHasTag` OtherComp "PlayerHitBox")
    (`/Engine/EditorBlueprintResources/StandardMacros.DoOnce` false
      (:`Completed`
        (set `self.CurrentDialogue` 0)
        (message `/Game/Blueprints/SystemDialogue/Interfaces/BPI_DialogueInfo.ResetDialogue` (`GameplayStatics.GetPlayerPawn` 0))
        (`KismetSystemLibrary.DelayUntilNextTick`)
        (`/Engine/EditorBlueprintResources/StandardMacros.DoOnce` false :!label _label
          (:`Completed`
            (`self.Speaking`)
            (if (>= (`self.CurrentDialogue`) (`KismetArrayLibrary.Array_Length` _dialoguedataasset))
              (`KismetSystemLibrary.Delay` _returnvalue)
              (`KismetSystemLibrary.Delay` 2.0)
              (message `/Game/Blueprints/SystemDialogue/Interfaces/BPI_DialogueInfo.HideDialogue` (`GameplayStatics.GetPlayerPawn` 0))
              (`self.K2_DestroyActor`)
              (else
                (`KismetSystemLibrary.Delay` _returnvalue)
                (`|ExecutionSequence`
                  (:`then_0`
                    (goto _label :!via `Reset`))
                  (:`then_1`
                    (goto _label)))))))))))

(fn `SetAllVariables`
  (params (InputPin :type "/Game/Blueprints/SystemDialogue/Outdated/PDA_LigneDialogue Object Reference") (S_DialogueInfoTree :type "/Game/Blueprints/SystemDialogue/Outdated/S_DialogueInfoTree Structure (by ref)"))
  (bind (_id _dialogue _dialoguefontinfo _dialoguetextcolor _charactername _characternamefontinfo _characternametextcolor _soundtoplay _minpitch _maxpitch _voicevolumemultiplier _characterimage _timebeforeskip _blockplayermovement_ _islastline_ _textspeed) (break `/Game/Blueprints/SystemDialogue/Outdated/S_DialogueInfoTree` S_DialogueInfoTree))
  (`|ExecutionSequence`
    (:`then_0`
      (set `/Game/Blueprints/SystemDialogue/Outdated/PDA_LigneDialogue.DialogueText` _dialogue InputPin))
    (:`then_1`
      (set `/Game/Blueprints/SystemDialogue/Outdated/PDA_LigneDialogue.DialogueFontInfo` _dialoguefontinfo InputPin))
    (:`then_2`
      (set `/Game/Blueprints/SystemDialogue/Outdated/PDA_LigneDialogue.DialogueTextColor` _dialoguetextcolor InputPin))
    (:`then_3`
      (set `/Game/Blueprints/SystemDialogue/Outdated/PDA_LigneDialogue.CharacterName` _charactername InputPin))
    (:`then_4`
      (set `/Game/Blueprints/SystemDialogue/Outdated/PDA_LigneDialogue.CharacterNameFontInfo` _characternamefontinfo InputPin))
    (:`then_5`
      (set `/Game/Blueprints/SystemDialogue/Outdated/PDA_LigneDialogue.CharacterTextColor` _characternametextcolor InputPin))
    (:`then_6`
      (set `/Game/Blueprints/SystemDialogue/Outdated/PDA_LigneDialogue.MinPitch` _minpitch InputPin))
    (:`then_7`
      (set `/Game/Blueprints/SystemDialogue/Outdated/PDA_LigneDialogue.MaxPitch` _maxpitch InputPin))
    (:`then_8`
      (set `/Game/Blueprints/SystemDialogue/Outdated/PDA_LigneDialogue.VoiceVolumeMultiplier` _voicevolumemultiplier InputPin))
    (:`then_9`
      (set `/Game/Blueprints/SystemDialogue/Outdated/PDA_LigneDialogue.CharacterImage` _characterimage InputPin))
    (:`then_10`
      (set `/Game/Blueprints/SystemDialogue/Outdated/PDA_LigneDialogue.TimeBeforeSkip` _timebeforeskip InputPin))
    (:`then_11`
      (set `/Game/Blueprints/SystemDialogue/Outdated/PDA_LigneDialogue.BlockPlayerMovement?` _blockplayermovement_ InputPin))
    (:`then_12`
      (set `/Game/Blueprints/SystemDialogue/Outdated/PDA_LigneDialogue.IsLastLine?` _islastline_ InputPin))
    (:`then_13`
      (set `/Game/Blueprints/SystemDialogue/Outdated/PDA_LigneDialogue.TextSpeed` _textspeed InputPin))))

(fn `Speaking`
  (bind _returnvalue (`GameplayStatics.GetPlayerPawn` 0))
  (bind _dialoguedataasset (`self.DialogueDataAsset`))
  (bind _isspeaking_ (message `/Game/Blueprints/SystemDialogue/Interfaces/BPI_DialogueInfo.CheckSpeaking` _returnvalue))
  (if (not _isspeaking_)
    (message `/Game/Blueprints/SystemDialogue/Interfaces/BPI_DialogueInfo.Speaking` _returnvalue (`|GetArrayItem` _dialoguedataasset (`self.CurrentDialogue`)) self)
    (bind _result (`/Engine/EditorBlueprintResources/StandardMacros.IncrementInt` (`self.CurrentDialogue`))
      (:`  `
        (`|ExecutionSequence`
          (:`then_0`
            (return))
          (:`then_1`
            (if (and (not _isspeaking_) (>= _result (`KismetArrayLibrary.Array_Length` _dialoguedataasset)))
              (`self.K2_DestroyActor`))))))))

(fn `UpdateDialogue `
  (bind _outassetdata (`AssetRegistry.GetAssetsByPath` (`AssetRegistryHelpers.GetAssetRegistry`) "/Game/Blueprints/SystemDialogue/DataAssets/DataAssetReader" false false))
  (for _array_element _outassetdata
    (bind _aspda_ligne_dialogue (cast `/Game/Blueprints/SystemDialogue/Outdated/PDA_LigneDialogue` (`AssetRegistryHelpers.GetAsset` _array_element)))
    (bind _returnvalue (`|GetDataTableRow` "/Game/Blueprints/SystemDialogue/Outdated/TableDialogue.TableDialogue" (`KismetStringLibrary.Conv_StringToName` (`KismetStringLibrary.Conv_IntToString` (`/Game/Blueprints/SystemDialogue/Outdated/PDA_LigneDialogue.Id` _aspda_ligne_dialogue))))
      (:`then`
        (`self.SetAllVariables` _aspda_ligne_dialogue _returnvalue)))))

(fn `UserConstructionScript`)