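; Blueprint function library whose PaintOnMesh function paints colored splashes onto BP_ParentCanvas actors.
; A supplied line trace or a short camera-forward trace finds the impact point, where a multi-sphere trace gathers the surfaces within brush range.
; Each canvas hit draws at its UV channel 1 location, with brush size shrunk by distance from impact like a sphere's cross-section.
; Averaged actor scale is passed along, which the author notes only suits equal-sided shapes.
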(fn `PaintOnMesh`
  (params (Radius :type "Float (double-precision)") (PaintColor :type "LinearColor Structure") (LineTraceStart :type "Vector Structure") (LineTraceEnd :type "Vector Structure") (HasExternalTrace :type Boolean))
  (locals (BrushSize :type "Float (double-precision)" :default 500.0) (HitResult :type "HitResult Structure"))
  (bind _returnvalue (`GameplayStatics.GetPlayerCameraManager` null))
  (bind (_bblockinghit _binitialoverlap _time _distance _location _impactpoint) (`GameplayStatics.BreakHitResult` (`local.HitResult`)))
  (bind _returnvalue_2 (`PlayerCameraManager.GetCameraLocation` _returnvalue))
  (set `local.BrushSize` Radius)
  (if HasExternalTrace
    ; Ray trace externe
    (bind _outhit (`KismetSystemLibrary.LineTraceSingle` :`Start` (`local.LineTraceStart`) :`End` (`local.LineTraceEnd`) :`TraceChannel` "TraceTypeQuery1" :`bTraceComplex` true :`TraceColor` (struct :`B` 1.0 :`A` 1.0)))
    (set `local.HitResult` _outhit)
    (else
      ; Ray trace normal
      (bind _outhit_2 (`KismetSystemLibrary.LineTraceSingle` :`Start` _returnvalue_2 :`End` (+ _returnvalue_2 (* (`Actor.GetActorForwardVector` _returnvalue) 500.0)) :`TraceChannel` "TraceTypeQuery1" :`bTraceComplex` true :`TraceColor` (struct :`G` 1.0 :`B` 1.0 :`A` 1.0)))
      (set `local.HitResult` _outhit_2)))
  ; Zone d'impact du pinceau
  (bind _outhits (`KismetSystemLibrary.SphereTraceMulti` null _impactpoint _impactpoint (/ (`local.BrushSize`) 20.48) "TraceTypeQuery1" true))
  (for _array_element _outhits
    (bind (_bblockinghit_2 _binitialoverlap_2 _time_2 _distance_2 _location_2 _impactpoint_2 _normal _impactnormal _physmat _hitactor) (`GameplayStatics.BreakHitResult` _array_element))
    (bind _asbp_parent_canvas (cast `/Game/Blueprints/Painting/PaintType1_Canvas/BP_ParentCanvas` _hitactor))
    (bind (_returnvalue_x _returnvalue_y _returnvalue_z) (`KismetMathLibrary.BreakVector` (`Actor.GetActorScale3D` _hitactor)))
    (`/Game/Blueprints/Painting/PaintType1_Canvas/BP_ParentCanvas.DrawBrushCanvas` _asbp_parent_canvas "/Game/Blueprints/Painting/Other/PaintSplash_Tex.PaintSplash_Tex" (`KismetMathLibrary.Sqrt` (- (`KismetMathLibrary.Square` (`local.BrushSize`)) (`KismetMathLibrary.Square` (* (`KismetMathLibrary.Vector_Distance` _impactpoint_2 _impactpoint) 20.48)))) (`GameplayStatics.FindCollisionUV` _array_element 1) PaintColor (/ (+ _returnvalue_x _returnvalue_y _returnvalue_z) 3.0))))