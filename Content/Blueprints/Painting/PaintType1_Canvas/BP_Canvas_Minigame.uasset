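; Painting canvas minigame actor that lets the player toggle into a mouse-driven painting view via Interact.
; A trigger box shows or hides the interact prompt, while Interact finds BP_Painter, blends the view to CameraActor or back, and toggles the cursor.
; During the minigame, Tick overrides the painter's line trace with one from the camera through the deprojected mouse position.
; The logic that spawns CameraActor at the Arrow is disconnected.
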(event `self.ReceiveTick`
  (params (DeltaSeconds :type "Float (single-precision)"))
  (bind _bp_painter (`self.BP_Painter`))
  (bind (_worldlocation _worlddirection) (`PlayerController.DeprojectMousePositionToWorld` (`GameplayStatics.GetPlayerController` 0)))
  (`parent.ReceiveTick` DeltaSeconds)
  (if (`self.IsInMinigame`)
    (set `/Game/Blueprints/Painting/PaintType1_Canvas/BP_Painter.Line Trace Start` (`self.K2_GetActorLocation` (`self.CameraActor`)) _bp_painter)
    (set `/Game/Blueprints/Painting/PaintType1_Canvas/BP_Painter.Line Trace End` (+ _worldlocation (* _worlddirection 1000.0)) _bp_painter)
    (set `/Game/Blueprints/Painting/PaintType1_Canvas/BP_Painter.Has External Trace` true _bp_painter)))

(event `self.ReceiveBeginPlay`
  (`parent.ReceiveBeginPlay`))

(event `/Game/Blueprints/LVL_Artiste3D/BlueprintActor/BPI_Interactable.Interact`
  (bind _returnvalue (`GameplayStatics.GetPlayerController` 0))
  (`Widget.SetVisibility` (`self.WBP_Interact`) "Collapsed")
  (bind _returnvalue_2 (`GameplayStatics.GetActorOfClass` "/Game/Blueprints/Painting/PaintType1_Canvas/BP_Painter.BP_Painter_C"))
  (set `self.BP_Painter` _returnvalue_2)
  (if (`self.IsInMinigame`)
    (set `self.IsInMinigame` false)
    (`PlayerController.SetViewTargetWithBlend` _returnvalue _returnvalue 0.5 "VTBlend_Linear" 0.0 false)
    (set `PlayerController.bShowMouseCursor` false (`GameplayStatics.GetPlayerController` 0))
    (else
      (set `self.IsInMinigame` true)
      (`PlayerController.SetViewTargetWithBlend` (`GameplayStatics.GetPlayerController` 0) (`self.CameraActor`) 0.5 "VTBlend_Linear" 0.0 false)
      (set `PlayerController.bShowMouseCursor` true (`GameplayStatics.GetPlayerController` 0)))))

(event `self.TriggerBox.OnComponentBeginOverlap`
  (params (OverlappedComponent :type "PrimitiveComponent Object Reference") (OtherActor :type "Actor Object Reference") (OtherComp :type "PrimitiveComponent Object Reference") (OtherBodyIndex :type Integer) (bFromSweep :type Boolean) (SweepResult :type "HitResult Structure (by ref)"))
  (`/Engine/EditorBlueprintResources/StandardMacros.IsValid` (`self.WBP_Interact`)
    (:`Is Valid`
      _)
    (:`Is Not Valid`
      (bind _returnvalue (`|CreateWidget` "/Game/UI/Widgets/W_InteractPrompt.W_InteractPrompt_C"))
      (set `self.WBP_Interact` _returnvalue)))
  (`Widget.SetVisibility` (`self.WBP_Interact`) "Visible"))

(event `self.TriggerBox.OnComponentEndOverlap`
  (params (OverlappedComponent :type "PrimitiveComponent Object Reference") (OtherActor :type "Actor Object Reference") (OtherComp :type "PrimitiveComponent Object Reference") (OtherBodyIndex :type Integer))
  (`Widget.SetVisibility` (`self.WBP_Interact`) "Collapsed"))

(fn `UserConstructionScript`
  (`parent.UserConstructionScript`))