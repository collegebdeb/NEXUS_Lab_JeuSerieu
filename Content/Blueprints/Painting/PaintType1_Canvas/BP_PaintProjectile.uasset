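; Paint projectile that takes its color from BP_Painter, paints the mesh it hits and bursts into a colored Niagara splash.
; BeginPlay predicts the impact point along the camera's forward vector, skipping ignored actor classes.
; Reaching that point or a component hit triggers Hit.
; Hit sphere-traces for the surface, calls PaintOnMesh with line traces in both directions through it, then destroys the projectile.
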(event `AllActorsToIgnore`
  (for _array_element (`self.ActorClassesToIgnore`)
    (bind _outactors (`GameplayStatics.GetAllActorsOfClass` _array_element))
    (for _array_element_2 _outactors
      (`KismetArrayLibrary.Array_Add` (`self.Actors To Ignore`) _array_element_2))))

(event `self.ReceiveBeginPlay`
  (`self.AllActorsToIgnore`)
  (bind _predictresult (`GameplayStatics.Blueprint_PredictProjectilePath_Advanced` (make `PredictProjectilePathParams` :`StartLocation` (`SceneComponent.K2_GetComponentLocation` (`self.Projectile`)) :`LaunchVelocity` (* (`SceneComponent.GetForwardVector` (`PlayerCameraManager.TransformComponent` (`PlayerController.PlayerCameraManager` (`GameplayStatics.GetPlayerController` 0)))) (`ProjectileMovementComponent.InitialSpeed` (`self.ProjectileMovement`))) :`bTraceWithCollision` true :`ProjectileRadius` 30.0 :`TraceChannel` "ECC_GameTraceChannel1" :`ActorsToIgnore` (`self.Actors To Ignore`) :`bTraceComplex` true)))
  (`KismetSystemLibrary.DelayUntilNextTick`)
  (bind _returnvalue (`GameplayStatics.GetActorOfClass` "/Game/Blueprints/Painting/PaintType1_Canvas/BP_Painter.BP_Painter_C"))
  (set `self.BP_Painter` _returnvalue)
  (bind _bp_painter (`self.BP_Painter`)
    (:`then`
      (bind _output_get (set `self.Paint Color` (`/Game/Blueprints/Painting/PaintType1_Canvas/BP_Painter.Paint Color` _bp_painter)))
      (`MeshComponent.SetColorParameterValueOnMaterials` (`self.Projectile`) "Color" _output_get))
    (:`else`)))

(event `self.ReceiveTick`
  (params (DeltaSeconds :type "Float (single-precision)"))
  (if (== (`SceneComponent.K2_GetComponentLocation` (`self.Projectile`)) (`.ImpactPoint` (`GameplayStatics.BreakHitResult` (`.HitResult` (break `PredictProjectilePathResult` (stale `self.ReceiveBeginPlay` _predictresult))))) :`ErrorTolerance` 30.0)
    (`self.Hit`)))

(event `self.Projectile.OnComponentHit`
  (params (HitComponent :type "PrimitiveComponent Object Reference") (OtherActor :type "Actor Object Reference") (OtherComp :type "PrimitiveComponent Object Reference") (NormalImpulse :type "Vector Structure") (Hit :type "HitResult Structure (by ref)"))
  (`KismetSystemLibrary.DelayUntilNextTick`)
  (`self.Hit`))

(event `Hit`
  (bind _returnvalue (`self.K2_GetActorLocation` self))
  (bind _returnvalue_2 (+ (`self.K2_GetActorLocation` self) (* (`self.GetActorForwardVector` self) -5.0)))
  (bind _outhit (`KismetSystemLibrary.SphereTraceSingle` _returnvalue _returnvalue (`self.Projectile_SplashRadius`) "TraceTypeQuery1" true))
  (bind _returnvalue_3 (- _returnvalue_2 (* (- _returnvalue_2 (`.ImpactPoint` (`GameplayStatics.BreakHitResult` _outhit))) 5.0)))
  (`/Game/Blueprints/Painting/BPFL_Utilities.PaintOnMesh` (* (`self.Projectile_SplashRadius`) 100.0) (`self.Paint Color`) _returnvalue_2 _returnvalue_3 true)
  (`/Game/Blueprints/Painting/BPFL_Utilities.PaintOnMesh` (* (`self.Projectile_SplashRadius`) 100.0) (`self.Paint Color`) _returnvalue_3 _returnvalue_2 true)
  (bind _returnvalue_4 (`NiagaraFunctionLibrary.SpawnSystemAtLocation` "/Game/Art/Niagara/P_B_splash_Variable.P_B_splash_Variable" (`self.K2_GetActorLocation` self)))
  (`NiagaraComponent.SetVariableLinearColor` _returnvalue_4 "SplashColor" (`self.Paint Color`))
  (`self.K2_DestroyActor`))

(fn `UserConstructionScript`)