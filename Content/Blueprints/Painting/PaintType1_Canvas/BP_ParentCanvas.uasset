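; BP_ParentCanvas is a paintable canvas that stores brush strokes in a render target.
; On BeginPlay it creates and clears a 4K render target, feeds it to a dynamic Canvas_Mat on the Canvas component, and creates a dynamic brush material.
; DrawBrushCanvas sets brush texture and color, then draws that material into the render target at a normalized location, dividing brush size by actor scale.
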(event `self.ReceiveBeginPlay`
  (`|ExecutionSequence`
    (:`then_0`
      (bind _returnvalue (`KismetRenderingLibrary.CreateRenderTarget2D` 4096 4096 "RTF_RGBA16f" (struct :`R` 1.0 :`G` 1.0 :`B` 1.0 :`A` 1.0)))
      (bind _output_get (set `self.RenderTarget` _returnvalue))
      (`KismetRenderingLibrary.ClearRenderTarget2D` _output_get (struct :`R` 1.0 :`G` 1.0 :`B` 1.0)))
    (:`then_1`
      (bind _returnvalue_2 (`KismetMaterialLibrary.CreateDynamicMaterialInstance` "/Game/Blueprints/Painting/PaintType1_Canvas/Canvas_Mat.Canvas_Mat"))
      (for (_ _array_index) (`MeshComponent.GetMaterials` (`self.Canvas`))
        (`MaterialInstanceDynamic.SetTextureParameterValue` _returnvalue_2 "RenderTarget" (`self.RenderTarget`))
        (`PrimitiveComponent.SetMaterial` (`self.Canvas`) _array_index _returnvalue_2)))
    (:`then_2`
      (bind _returnvalue_3 (`KismetMaterialLibrary.CreateDynamicMaterialInstance` "/Game/Blueprints/Painting/Other/M_Brush.M_Brush"))
      (set `self.BrushMat` _returnvalue_3))))

(fn `DrawBrushCanvas`
  (params (BrushTexture :type "Texture2D Object Reference") (BrushSize :type "Float (double-precision)") (DrawLocation :type "Vector2D Structure") (BrushColor :type "LinearColor Structure") (ActorScale :type "Float (double-precision)"))
  (bind _brushmat (`self.BrushMat`))
  (bind _returnvalue (/ (`local.BrushSize`) ActorScale))
  (`|ExecutionSequence`
    (:`then_0`
      (`MaterialInstanceDynamic.SetTextureParameterValue` _brushmat "BrushTexture" BrushTexture)
      (`MaterialInstanceDynamic.SetVectorParameterValue` _brushmat "Hue" BrushColor))
    (:`then_1`
      (bind (_canvas _size _context) (`KismetRenderingLibrary.BeginDrawCanvasToRenderTarget` (`self.RenderTarget`)))
      (`Canvas.K2_DrawMaterial` _canvas (`self.BrushMat`) (- (* _size (`local.DrawLocation`)) (/ (`local.BrushSize`) (* ActorScale 2.0))) (`KismetMathLibrary.MakeVector2D` _returnvalue _returnvalue) (0.0 0.0) (1.0 1.0) 0.0 (0.5 0.5))
      (`KismetRenderingLibrary.EndDrawCanvasToRenderTarget` _context))))

(fn `UserConstructionScript`)