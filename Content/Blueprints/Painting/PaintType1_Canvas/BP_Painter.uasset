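; BP_Painter is the Type 1 canvas painter, calling PaintOnMesh every tick with the current radius and color.
; Paint events step the radius and alpha up or down and cycle the color through DTPaintColor rows, looked up by wrapping index.
; ColorAlpha only reaches PaintColor at BeginPlay; later alpha steps do not update it, and color changes use the table's own alpha.
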(event `self.ReceiveBeginPlay`
  ; Set color to first
  (bind _returnvalue (`|GetDataTableRow` (`self.DT_PaintColor`) (`KismetStringLibrary.Conv_StringToName` (`KismetStringLibrary.Conv_IntToString` (`self.Table_Position`))))
    (:`then`
      (bind (_name _color) (break `/Game/Blueprints/Painting/PaintType1_Canvas/STR_Colors` _returnvalue))
      (set `self.Paint Color` (make `LinearColor` (break `LinearColor` _color) (`.G` (break `LinearColor` _color)) (`.B` (break `LinearColor` _color)) (`self.Color_Alpha`)))
      ; Get data table length
      (bind _outrownames (`DataTableFunctionLibrary.GetDataTableRowNames` (`self.DT_PaintColor`)))
      (set `self.DT_Length` (`KismetArrayLibrary.Array_Length` _outrownames)))))

(event `self.ReceiveTick`
  (params (DeltaSeconds :type "Float (single-precision)"))
  ; Type1_Painting
  (`/Game/Blueprints/Painting/BPFL_Utilities.PaintOnMesh` (`self.Paint_Radius`) (`self.Paint Color`)))

(event `Paint_Size_IncrementDown`
  ; Reduce paint radius
  (set `self.Paint_Radius` (- (`self.Paint_Radius`) (`self.Paint_Radius_Multiplier`))))

(event `Paint_Size_IncrementUp`
  ; Up paint radius
  (set `self.Paint_Radius` (+ (`self.Paint_Radius`) (`self.Paint_Radius_Multiplier`))))

(event `Paint_Color_Change`
  ; Change color
  (bind _result (`/Engine/EditorBlueprintResources/StandardMacros.IncrementInt` (`self.Table_Position`))
    (:`  `
      (bind _output_get (set `self.Table_Position` (mod _result (`self.DT_Length`))))
      ; Set color
      (bind _returnvalue (`|GetDataTableRow` (`self.DT_PaintColor`) (`KismetStringLibrary.Conv_StringToName` (`KismetStringLibrary.Conv_IntToString` _output_get)))
        (:`then`
          (set `self.Paint Color` (`.Color_2_53DE62814B0B53C6911BB698D1B71F66` (break `/Game/Blueprints/Painting/PaintType1_Canvas/STR_Colors` _returnvalue))))))))

(event `Paint_AlphaChannel_IncrementDown`
  ; Reduce paint alpha
  (set `self.Color_Alpha` (- (`self.Color_Alpha`) (`self.Color_Alpha_Multiplier`))))

(event `Paint_AlphaChannel_IncrementUp`
  ; Up paint alpha
  (set `self.Color_Alpha` (+ (`self.Color_Alpha`) (`self.Color_Alpha_Multiplier`))))

(fn `UserConstructionScript`)