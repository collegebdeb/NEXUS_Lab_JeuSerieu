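; Paint area trigger volume that supplies a BP_Paintbrush and ends painting when the player leaves.
; On BeginPlay it spawns the brush at PaintbrushSpawnpoint and keeps a reference to it.
; When BP_FirstPersonCharacter exits the box, it disables paint throwing and hides top-level WBP_Painting widgets.
; Within that widget loop, a missing brush is respawned and the player's HeldItem mesh is cleared.
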(event `self.ReceiveBeginPlay`
  (bind _returnvalue (`|SpawnActorFromClass` "/Game/Blueprints/Painting/BP_Paintbrush.BP_Paintbrush_C" (`KismetMathLibrary.MakeTransform` (`SceneComponent.K2_GetComponentLocation` (`self.PaintbrushSpawnpoint`))) "Undefined" "MultiplyWithRoot" null null))
  (set `self.LocalPaintbrush` _returnvalue))

(event `self.Box.OnComponentEndOverlap`
  (params (OverlappedComponent :type "PrimitiveComponent Object Reference") (OtherActor :type "Actor Object Reference") (OtherComp :type "PrimitiveComponent Object Reference") (OtherBodyIndex :type Integer))
  (bind (_asbp_first_person_character _bsuccess) (cast `/Game/FirstPerson/Blueprints/BP_FirstPersonCharacter` OtherActor :!pure true))
  (if _bsuccess
    (set `/Game/FirstPerson/Blueprints/BP_FirstPersonCharacter.CanThrowPaint` false _asbp_first_person_character)
    (bind _foundwidgets (`WidgetBlueprintLibrary.GetAllWidgetsOfClass` "/Game/UI/Widgets/WBP_Painting.WBP_Painting_C"))
    (for _array_element _foundwidgets
      (`Widget.SetVisibility` _array_element "Hidden")
      (`/Engine/EditorBlueprintResources/StandardMacros.IsValid` (`self.LocalPaintbrush`)
        (:`Is Not Valid`
          (bind _returnvalue (`|SpawnActorFromClass` "/Game/Blueprints/Painting/BP_Paintbrush.BP_Paintbrush_C" (`KismetMathLibrary.MakeTransform` (`SceneComponent.K2_GetComponentLocation` (`self.PaintbrushSpawnpoint`))) "Undefined" "MultiplyWithRoot" null null))
          (set `self.LocalPaintbrush` _returnvalue)
          (bind _asbp_first_person_character_2 (cast `/Game/FirstPerson/Blueprints/BP_FirstPersonCharacter` (`GameplayStatics.GetPlayerPawn` 0)))
          (`StaticMeshComponent.SetStaticMesh` (`/Game/FirstPerson/Blueprints/BP_FirstPersonCharacter.Held_Item` _asbp_first_person_character_2) null))))))

(fn `UserConstructionScript`)