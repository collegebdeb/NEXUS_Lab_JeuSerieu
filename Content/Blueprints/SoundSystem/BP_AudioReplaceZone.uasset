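; BP_AudioReplaceZone is a zone actor that swaps one of the game's audio tracks when the first-person player character enters it.
; On BeginPlay it finds and caches the BP_AudioManager in the level.
; On overlap it uses TrackToReplace to choose the manager's main or secondary audio track and sets that component's sound to NewAudioTrack.
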(event `self.ReceiveBeginPlay`
  (bind _returnvalue (`GameplayStatics.GetActorOfClass` "/Game/Blueprints/SoundSystem/BP_AudioManager.BP_AudioManager_C"))
  (set `self.AudioManager` _returnvalue))

(event `self.ReceiveActorBeginOverlap`
  (params (OtherActor :type "Actor Object Reference"))
  (bind _audiomanager (`self.AudioManager`))
  (bind _newaudiotrack (`self.NewAudioTrack`))
  (cast `/Game/FirstPerson/Blueprints/BP_FirstPersonCharacter` OtherActor)
  (switch `/Game/Blueprints/SoundSystem/ENUM_MainSecondary` (`self.TrackToReplace`)
    (:`NewEnumerator0`
      (`AudioComponent.SetSound` (`/Game/Blueprints/SoundSystem/BP_AudioManager.MainAudioTrack` _audiomanager) _newaudiotrack))
    (:`NewEnumerator1`
      (`AudioComponent.SetSound` (`/Game/Blueprints/SoundSystem/BP_AudioManager.SecondaryAudioTrack` _audiomanager) _newaudiotrack))))

(fn `UserConstructionScript`)