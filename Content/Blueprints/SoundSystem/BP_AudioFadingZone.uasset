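; BP_AudioFadingZone is a box zone that crossfades soundtracks as the first-person character moves through it.
; Overlap events toggle IsActive, which gates the fade on Tick.
; Tick derives entrance and exit points from the box's forward axis, then measures player progress using world X only.
; That progress, shaped by an attenuation exponent, fades entrance tracks out and exit tracks in through BP_AudioManager's components, with debug drawing and printing.
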(event `self.ReceiveBeginPlay`
  (bind _returnvalue (`GameplayStatics.GetActorOfClass` "/Game/Blueprints/SoundSystem/BP_AudioManager.BP_AudioManager_C"))
  (set `self.AudioManager` _returnvalue))

(event `self.ReceiveActorBeginOverlap`
  (params (OtherActor :type "Actor Object Reference"))
  (cast `/Game/FirstPerson/Blueprints/BP_FirstPersonCharacter` OtherActor)
  (set `self.IsActive` true))

(event `self.ReceiveActorEndOverlap`
  (params (OtherActor :type "Actor Object Reference"))
  (cast `/Game/FirstPerson/Blueprints/BP_FirstPersonCharacter` OtherActor)
  (set `self.IsActive` false))

(event `self.ReceiveTick`
  (params (DeltaSeconds :type "Float (single-precision)"))
  (bind _returnvalue (`self.GetActorScale3D`))
  (bind _returnvalue_2 (`self.K2_GetActorRotation`))
  (bind _returnvalue_3 (`self.GetActorScale3D`))
  (bind _returnvalue_4 (`self.K2_GetActorRotation`))
  (bind _atenuationstrength (`self.AtenuationStrength`))
  (bind _triggerentrance (`self.TriggerEntrance`))
  (bind _returnvalue_x (`KismetMathLibrary.BreakVector` (- (`self.TriggerExit`) _triggerentrance)))
  (bind (_boxextent_x _boxextent_y _boxextent_z) (`KismetMathLibrary.BreakVector` (`BoxComponent.BoxExtent` (`self.Box`))))
  (bind (_boxextent_x_2 _boxextent_y_2 _boxextent_z_2) (`KismetMathLibrary.BreakVector` (`BoxComponent.BoxExtent` (`self.Box`))))
  (bind _returnvalue_x_2 (`KismetMathLibrary.BreakVector` (- (`self.K2_GetActorLocation` (`GameplayStatics.GetPlayerPawn` 0)) _triggerentrance)))
  (bind _returnvalue_5 (+ (`self.K2_GetActorLocation`) (* _returnvalue (`KismetMathLibrary.GetForwardVector` _returnvalue_2) (`KismetMathLibrary.MakeVector` _boxextent_x _boxextent_x _boxextent_x))))
  (bind _returnvalue_6 (/ _returnvalue_x_2 _returnvalue_x))
  (bind _returnvalue_7 (- (`self.K2_GetActorLocation`) (* _returnvalue_3 (`KismetMathLibrary.GetForwardVector` _returnvalue_4) (`KismetMathLibrary.MakeVector` _boxextent_x_2 _boxextent_x_2 _boxextent_x_2))))
  (set `self.TriggerEntrance` _returnvalue_7)
  (`KismetSystemLibrary.DrawDebugBox` _returnvalue_7 (* _returnvalue_3 (`KismetMathLibrary.MakeVector` 100.0 _boxextent_y_2 _boxextent_z_2)) (struct :`G` 1.0 :`A` 1.0) _returnvalue_4 0.0 10.0)
  (set `self.TriggerExit` _returnvalue_5)
  (`KismetSystemLibrary.DrawDebugBox` _returnvalue_5 (* _returnvalue (`KismetMathLibrary.MakeVector` 100.0 _boxextent_y _boxextent_z)) (struct :`R` 1.0 :`B` 1.0 :`A` 1.0) _returnvalue_2 0.0 10.0)
  (`self.IsActive`
    (:`then`
      (set `self.CompletionPercent` (`KismetMathLibrary.FClamp` _returnvalue_6 0.0))
      (`KismetSystemLibrary.PrintString` (`KismetStringLibrary.Conv_DoubleToString` _returnvalue_6) true true (struct :`R` 0.293121 :`G` 1.0 :`A` 1.0) 0.0)
      (`|ExecutionSequence`
        (:`then_0`
          (for _array_element (`self.AudioAtEntrance`)
            (`AudioComponent.SetVolumeMultiplier` (`BlueprintMapLibrary.Map_Find` (`/Game/Blueprints/SoundSystem/BP_AudioManager.SoundTracksComponents` (`self.AudioManager`)) _array_element) (`KismetMathLibrary.MultiplyMultiply_FloatFloat` (`KismetMathLibrary.MapRangeClamped` (`self.CompletionPercent`) 0.0 1.0 1.0) _atenuationstrength))))
        (:`then_1`
          (for _array_element_2 (`self.AudioAtExit`)
            (`AudioComponent.SetVolumeMultiplier` (`BlueprintMapLibrary.Map_Find` (`/Game/Blueprints/SoundSystem/BP_AudioManager.SoundTracksComponents` (`self.AudioManager`)) _array_element_2) (`KismetMathLibrary.MultiplyMultiply_FloatFloat` (`self.CompletionPercent`) _atenuationstrength))))))
    (:`else`)))

(fn `UserConstructionScript`)