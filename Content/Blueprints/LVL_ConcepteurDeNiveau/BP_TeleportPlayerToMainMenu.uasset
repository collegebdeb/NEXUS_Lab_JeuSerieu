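; Trigger actor that ends the current level with a fade to black and dialogue, then returns the player to the main menu.
; Overlapping the trigger box starts a Tick-driven manual camera fade; once fully black, it queues a dialogue once through GM_FirstPerson.
; The OnEndOfLine event shows the loading widget, then opens the main menu level after a short delay.
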(event `self.TriggerBox.OnComponentBeginOverlap`
  (params (OverlappedComponent :type "PrimitiveComponent Object Reference") (OtherActor :type "Actor Object Reference") (OtherComp :type "PrimitiveComponent Object Reference") (OtherBodyIndex :type Integer) (bFromSweep :type Boolean) (SweepResult :type "HitResult Structure (by ref)"))
  (set `self.StartEnd` true))

(event `self.ReceiveTick`
  (params (DeltaSeconds :type "Float (single-precision)"))
  (if (`self.StartEnd`)
    (bind _output_get (set `self.CurrentFadeToBlack` (`KismetMathLibrary.FInterpTo_Constant` (`self.CurrentFadeToBlack`) 1.0 (`GameplayStatics.GetWorldDeltaSeconds`) 1.0)))
    (`PlayerCameraManager.SetManualCameraFade` (`GameplayStatics.GetPlayerCameraManager` 0) _output_get (struct :`A` 1.0) false)
    (if (== _output_get 1.0)
      (`/Engine/EditorBlueprintResources/StandardMacros.DoOnce` false
        (:`Completed`
          (bind _asgm_first_person (cast `/Game/FirstPerson/Blueprints/GM_FirstPerson` (`GameplayStatics.GetGameMode`)))
          (`/Game/FirstPerson/Blueprints/GM_FirstPerson.QueueDialogue` _asgm_first_person (`self.Dialogue Data`)))))))

(event `/Game/Blueprints/SystemDialogue/Interfaces/BPI_EventCallAtEndOfLine.OnEndOfLine`
  (bind _returnvalue (`|CreateWidget` "/Game/UI/Widgets/WBP_Loading.WBP_Loading_C"))
  (`UserWidget.AddToViewport` _returnvalue 0)
  (`KismetSystemLibrary.Delay` 2.0)
  (`GameplayStatics.OpenLevelBySoftObjectPtr` "/Game/Levels/Menus_UI/L_Menu_Principal.L_Menu_Principal"))

(fn `UserConstructionScript`)