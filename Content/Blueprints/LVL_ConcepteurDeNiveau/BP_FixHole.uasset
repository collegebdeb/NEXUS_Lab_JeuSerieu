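; BP_FixHole is a level trigger that reveals a hidden static mesh, presumably patching a hole, based on where the player pawn faces.
; Its construction script hides the referenced mesh and disables its collision.
; On overlap, it checks HasBeenInTrigger across all BP_FixHole instances, then conditionally starts a near-per-frame looping timer.
; The timer makes the mesh visible and solid once player yaw falls within a set range.
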(event `self.TriggerBox.OnComponentBeginOverlap`
  (params (OverlappedComponent :type "PrimitiveComponent Object Reference") (OtherActor :type "Actor Object Reference") (OtherComp :type "PrimitiveComponent Object Reference") (OtherBodyIndex :type Integer) (bFromSweep :type Boolean) (SweepResult :type "HitResult Structure (by ref)"))
  (bind _outactors (`GameplayStatics.GetAllActorsOfClass` "BP_FixHole_C"))
  (for _array_element _outactors
    (if (== (`/Game/Blueprints/LVL_ConcepteurDeNiveau/BP_FixHole.HasBeenInTrigger` _array_element) true)
      (set `self.HasBeenInTrigger` true)
      (break)))
  (`self.HasBeenInTrigger`
    (:`then`)
    (:`else`
      (`KismetSystemLibrary.K2_SetTimerDelegate` (delegate `CustomEvent`) 1e-05 true true))))

(event `CustomEvent`
  (bind (_returnvalue_roll _returnvalue_pitch _returnvalue_yaw) (`KismetMathLibrary.BreakRotator` (`self.K2_GetActorRotation` (`GameplayStatics.GetPlayerPawn` 0))))
  (bind _staticmeshcomponent (`StaticMeshActor.StaticMeshComponent` (`self.StaticMeshToMakeAppear`)))
  (if (and (<= _returnvalue_yaw 131.0) (>= _returnvalue_yaw 5.0))
    (`PrimitiveComponent.SetCollisionEnabled` _staticmeshcomponent "QueryAndPhysics")
    (`SceneComponent.SetHiddenInGame` _staticmeshcomponent false false)))

(fn `UserConstructionScript`
  (bind _staticmeshcomponent (`StaticMeshActor.StaticMeshComponent` (`self.StaticMeshToMakeAppear`)))
  (`PrimitiveComponent.SetCollisionEnabled` _staticmeshcomponent "NoCollision")
  (`SceneComponent.SetHiddenInGame` _staticmeshcomponent true false))