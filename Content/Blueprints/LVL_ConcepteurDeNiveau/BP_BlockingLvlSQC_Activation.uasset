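; Interactable TV-screen trigger that, once activated by the player, either plays a referenced level sequence or sends dialogue to the player pawn.
; An overlap volume shows and hides an interact prompt widget.
; Interaction fires once, turning the screen's emissive color green through a dynamic material instance and hiding the prompt.
; In sequence mode, the prompt is also disabled and the sequence actor is destroyed when playback finishes.
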(event `self.ReceiveBeginPlay`
  (bind _tvscreen (`self.TVScreen`))
  ; Create dynamic material instance so the tv screen can change color
  (bind _returnvalue (`PrimitiveComponent.CreateDynamicMaterialInstance` _tvscreen 0 (`PrimitiveComponent.GetMaterial` _tvscreen 0) "None"))
  (set `self.DynamicTVSrceenMatInst` _returnvalue))

(event `self.UIPromptCollision.OnComponentBeginOverlap`
  (params (OverlappedComponent :type "PrimitiveComponent Object Reference") (OtherActor :type "Actor Object Reference") (OtherComp :type "PrimitiveComponent Object Reference") (OtherBodyIndex :type Integer) (bFromSweep :type Boolean) (SweepResult :type "HitResult Structure (by ref)"))
  ; Make visible the interact prompt
  (if (`self.CanWidgetBeVisible?`)
    (`SceneComponent.SetVisibility` (`self.W_InteractWidget`) true false)))

(event `self.UIPromptCollision.OnComponentEndOverlap`
  (params (OverlappedComponent :type "PrimitiveComponent Object Reference") (OtherActor :type "Actor Object Reference") (OtherComp :type "PrimitiveComponent Object Reference") (OtherBodyIndex :type Integer))
  ; Make visible the interact prompt
  (`SceneComponent.SetVisibility` (`self.W_InteractWidget`) false false))

(event `/Game/Blueprints/LVL_ConcepteurDeNiveau/Interfaces/BPI_InteractInfo.StartInteraction`
  (bind _sequenceplayer (`LevelSequenceActor.SequencePlayer` (`self.LevelSequenceReference`)))
  ; When player has pressed the interact key start the sequence
  (`/Engine/EditorBlueprintResources/StandardMacros.DoOnce` false
    (:`Completed`
      (if (`self.UseLvlSequence?`)
        (`MovieSceneSequencePlayer.Play` _sequenceplayer)
        (`MaterialInstanceDynamic.SetVectorParameterValue` (`self.DynamicTVSrceenMatInst`) "Emissive Color" (struct :`G` 1.0))
        (set `self.CanWidgetBeVisible?` false)
        (`SceneComponent.SetVisibility` (`self.W_InteractWidget`) false false)
        (add `MovieSceneSequencePlayer.OnFinished` _sequenceplayer (delegate `OnFinished_Event`))
        (else
          (message `/Game/Blueprints/SystemDialogue/Interfaces/BPI_DialogueInfo.SpeakingEventCallGeneric` (`GameplayStatics.GetPlayerPawn` 0) (`self.Dialogue Data`))
          (`MaterialInstanceDynamic.SetVectorParameterValue` (`self.DynamicTVSrceenMatInst`) "Emissive Color" (struct :`G` 1.0))
          (`SceneComponent.SetVisibility` (`self.W_InteractWidget`) false false))))))

(event `OnFinished_Event`
  ; When player has pressed the interact key start the sequence
  (`self.K2_DestroyActor` (`self.LevelSequenceReference`)))

(fn `UserConstructionScript`)