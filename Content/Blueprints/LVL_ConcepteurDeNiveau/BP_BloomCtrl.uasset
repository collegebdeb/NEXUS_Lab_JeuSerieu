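; BP_BloomCtrl is a trigger actor that steps a post-process volume's bloom through preset levels as the player enters it.
; When a component tagged PlayerHitBox begins overlapping its Box, AddBloom writes the current BloomAmount array entry into the referenced PostProcessVolume's intensity setting.
; Each trigger then increments CurrentIndex, with no bounds check or wraparound on the array.
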(event `AddBloom`
  (bind _output (`|ConvertAsset` (`self.PostProcessVolume`)))
  (bind _structout (setmembers `PostProcessSettings` :`StructRef` (`PostProcessVolume.Settings` _output) :`BloomIntensity` (`|GetArrayItem` (`self.BloomAmount`) (`self.CurrentIndex`))))
  (set `PostProcessVolume.Settings` _structout _output)
  (`/Engine/EditorBlueprintResources/StandardMacros.IncrementInt` (`self.CurrentIndex`)))

(event `self.Box.OnComponentBeginOverlap`
  (params (OverlappedComponent :type "PrimitiveComponent Object Reference") (OtherActor :type "Actor Object Reference") (OtherComp :type "PrimitiveComponent Object Reference") (OtherBodyIndex :type Integer) (bFromSweep :type Boolean) (SweepResult :type "HitResult Structure (by ref)"))
  (if (`ActorComponent.ComponentHasTag` OtherComp "PlayerHitBox")
    (`self.AddBloom`)))

(fn `UserConstructionScript`)