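; Level-design actor that moves a configurable static mesh along a spline once a trigger is overlapped.
; The trigger destroys itself on overlap, then Tick advances a distance by Speed and sets the mesh's relative location from the spline.
; Optional FInterpTo easing ramps speed at the start and slows it past a set fraction of the spline.
; The construction script applies mesh and material and can place the mesh at the spline's end.
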(event `self.ReceiveTick`
  (params (DeltaSeconds :type "Float (single-precision)"))
  (if (`self.CanMove?`)
    (if (`self.InterpSpeedAtTheBeginning?`)
      (bind _returnvalue (`KismetMathLibrary.FInterpTo` (`self.Speed`) (`self.TargetSpeed`) (`GameplayStatics.GetWorldDeltaSeconds`) (`self.InterpSpeedBeginning`)))
      (set `self.Speed` _returnvalue))
    (set `self.Distance` (+ (* DeltaSeconds (`self.Speed`)) (`self.Distance`)))
    (if (`self.InterpSpeedAtEnd?`)
      (if (> (`self.Distance`) (* (`SplineComponent.GetSplineLength` (`self.Spline`)) (`self.StartSlowdownWhen`)))
        (set `self.InterpSpeedAtTheBeginning?` false)
        (bind _returnvalue_2 (`KismetMathLibrary.FInterpTo` (`self.Speed`) (`self.TargetSpeedSlowdown`) (`GameplayStatics.GetWorldDeltaSeconds`) (`self.InterpSpeedEnd`)))
        (set `self.Speed` _returnvalue_2)))
    (`SceneComponent.K2_SetRelativeTransform` (`self.StaticMesh`) (`KismetMathLibrary.MakeTransform` (.location (`SplineComponent.GetTransformAtDistanceAlongSpline` (`self.Spline`) (`self.Distance`) "Local" false)) (`KismetMathLibrary.MakeRotator` 0.0) (`SceneComponent.RelativeScale3D` (`self.StaticMesh`))) false false)))

(event `self.TriggerPoint_0.OnComponentBeginOverlap`
  (params (OverlappedComponent :type "PrimitiveComponent Object Reference") (OtherActor :type "Actor Object Reference") (OtherComp :type "PrimitiveComponent Object Reference") (OtherBodyIndex :type Integer) (bFromSweep :type Boolean) (SweepResult :type "HitResult Structure (by ref)"))
  (set `self.CanMove?` true)
  (`ActorComponent.K2_DestroyComponent` (`self.TriggerPoint_0`)))

(fn `F_PlaceMeshAtEndOfSpline`
  (bind _staticmesh (`self.StaticMesh`))
  (bind (_returnvalue_location _returnvalue_rotation) (`KismetMathLibrary.BreakTransform` (`SceneComponent.GetRelativeTransform` _staticmesh)))
  (bind _returnvalue_location_2 (`KismetMathLibrary.BreakTransform` (`SplineComponent.GetTransformAtDistanceAlongSpline` (`self.Spline`) (`SplineComponent.GetSplineLength` (`self.Spline`)) "Local" false)))
  ; Place Mesh at end of spline if desired
  (`SceneComponent.K2_SetRelativeTransform` (`self.StaticMesh`) (`KismetMathLibrary.MakeTransform` _returnvalue_location_2 _returnvalue_rotation (`SceneComponent.RelativeScale3D` _staticmesh)) false false))

(fn `UserConstructionScript`
  (`|ExecutionSequence`
    (:`then_0`
      (`StaticMeshComponent.SetStaticMesh` (`self.StaticMesh`) (`self.MeshToMove`))
      (`PrimitiveComponent.SetMaterial` (`self.StaticMesh`) 0 (`self.MeshMaterial`)))
    (:`then_1`
      (if (`self.SetMeshAtEndOfSpline`)
        (`self.F_PlaceMeshAtEndOfSpline`)))))