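; BP_StartMusique is a trigger actor that plays a sequence of music clips, one per activation.
; Overlapping IT1 sets the current clip at full volume and disables that trigger.
; OnEndOfLine fades volume linearly to zero on a looping timer, then waits a per-clip delay, re-arms IT1 and advances the index.
; Overlapping DestroyBox destroys the actor.
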(event `self.ReceiveBeginPlay`
  (`AudioComponent.SetVolumeMultiplier` (`self.Musique`) 0.0))

(event `self.IT1.OnComponentBeginOverlap`
  (params (OverlappedComponent :type "PrimitiveComponent Object Reference") (OtherActor :type "Actor Object Reference") (OtherComp :type "PrimitiveComponent Object Reference") (OtherBodyIndex :type Integer) (bFromSweep :type Boolean) (SweepResult :type "HitResult Structure (by ref)"))
  (`AudioComponent.SetSound` (`self.Musique`) (`|GetArrayItem` (`self.MusiqueClips`) (`self.CurrentClipIndex`)))
  (`AudioComponent.SetVolumeMultiplier` (`self.Musique`) 1.0)
  (`PrimitiveComponent.SetCollisionEnabled` (`self.IT1`) "NoCollision")
  (set `self.CurrentSoundVolume` 1.0))

(event `/Game/Blueprints/SystemDialogue/Interfaces/BPI_EventCallAtEndOfLine.OnEndOfLine`
  (bind _returnvalue (`KismetSystemLibrary.K2_SetTimerDelegate` (delegate `LerpSoundVolume`) 1e-05 true true)))

(event `LerpSoundVolume`
  (bind _returnvalue (`KismetMathLibrary.FInterpTo_Constant` (`self.CurrentSoundVolume`) 0.0 (`GameplayStatics.GetWorldDeltaSeconds`) 0.1))
  (bind _output_get (set `self.CurrentSoundVolume` _returnvalue))
  (`AudioComponent.SetVolumeMultiplier` (`self.Musique`) _output_get)
  (if (== 0.0 (`self.CurrentSoundVolume`))
    (`KismetSystemLibrary.K2_ClearAndInvalidateTimerHandle` (stale `/Game/Blueprints/SystemDialogue/Interfaces/BPI_EventCallAtEndOfLine.OnEndOfLine` _returnvalue))
    (`KismetSystemLibrary.Delay` (`|GetArrayItem` (`self.Delays`) (`self.CurrentClipIndex`)))
    (`PrimitiveComponent.SetCollisionEnabled` (`self.IT1`) "QueryOnly")
    (`/Engine/EditorBlueprintResources/StandardMacros.IncrementInt` (`self.CurrentClipIndex`))))

(event `self.DestroyBox.OnComponentBeginOverlap`
  (params (OverlappedComponent :type "PrimitiveComponent Object Reference") (OtherActor :type "Actor Object Reference") (OtherComp :type "PrimitiveComponent Object Reference") (OtherBodyIndex :type Integer) (bFromSweep :type Boolean) (SweepResult :type "HitResult Structure (by ref)"))
  (`self.K2_DestroyActor`))

(fn `UserConstructionScript`)