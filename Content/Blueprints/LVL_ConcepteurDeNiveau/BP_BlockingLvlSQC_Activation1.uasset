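; Interactable actor with an outlined Zeus component that triggers a one-time level sequence and dialogue.
; A collision component toggles the interact prompt widget on overlap while it is allowed to show.
; Interacting clears the outline overlay, hides the prompt, and through a DoOnce plays the referenced sequence and queues dialogue on GM_FirstPerson.
; The Level Sequence actor is destroyed when playback finishes.
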(event `self.ReceiveBeginPlay`)

(event `self.UIPromptCollision.OnComponentBeginOverlap`
  (params (OverlappedComponent :type "PrimitiveComponent Object Reference") (OtherActor :type "Actor Object Reference") (OtherComp :type "PrimitiveComponent Object Reference") (OtherBodyIndex :type Integer) (bFromSweep :type Boolean) (SweepResult :type "HitResult Structure (by ref)"))
  ; Make visible the interact prompt
  (if (`self.CanWidgetBeVisible?`)
    (`SceneComponent.SetVisibility` (`self.W_InteractWidget`) true false)))

(event `self.UIPromptCollision.OnComponentEndOverlap`
  (params (OverlappedComponent :type "PrimitiveComponent Object Reference") (OtherActor :type "Actor Object Reference") (OtherComp :type "PrimitiveComponent Object Reference") (OtherBodyIndex :type Integer))
  ; Make visible the interact prompt
  (`SceneComponent.SetVisibility` (`self.W_InteractWidget`) false false :!label _label))

(event `self.StartInteraction`
  (bind _sequenceplayer (`LevelSequenceActor.SequencePlayer` (`self.LevelSequenceReference`)))
  ; When player has pressed the interact key start the sequence
  (`MeshComponent.SetOverlayMaterial` (`self.Zeus`) null)
  (set `self.CanWidgetBeVisible?` false)
  (`|ExecutionSequence`
    (:`then_0`
      (goto _label))
    (:`then_1`
      (`/Engine/EditorBlueprintResources/StandardMacros.DoOnce` false
        (:`Completed`
          (`|ExecutionSequence`
            (:`then_0`
              (`MovieSceneSequencePlayer.Play` _sequenceplayer)
              (set `self.CanWidgetBeVisible?` false)
              (`SceneComponent.SetVisibility` (`self.W_InteractWidget`) false false)
              (add `MovieSceneSequencePlayer.OnFinished` _sequenceplayer (delegate `OnFinished_Event`)))
            (:`then_1`
              (bind _asgm_first_person (cast `/Game/FirstPerson/Blueprints/GM_FirstPerson` (`GameplayStatics.GetGameMode`)))
              (`/Game/FirstPerson/Blueprints/GM_FirstPerson.QueueDialogue` _asgm_first_person (`self.Dialogue Data`)))))))))

(event `OnFinished_Event`
  ; When player has pressed the interact key start the sequence
  (`self.K2_DestroyActor` (`self.LevelSequenceReference`)))

(fn `UserConstructionScript`
  (`MeshComponent.SetOverlayMaterial` (`self.Zeus`) "/Game/Art/Materials/Instance/M_Outline_Inst.M_Outline_Inst"))