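; BP_Painter is a painter that draws onto BP_Washable actors where the player camera is pointing.
; Every tick it runs a debug-drawn multi line trace and calls DrawToRenderTarget at each washable's impact point with a fixed brush size.
; Input events adjust PaintRadius and cycle PaintColor through four data table rows.
; Both values feed only a disconnected PaintOnMesh call, so they do not affect the active render-target drawing.
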(event `self.ReceiveBeginPlay`
  ; Set color to first
  (bind _returnvalue (`|GetDataTableRow` (`self.DT_PaintColor`) (`KismetStringLibrary.Conv_StringToName` (`KismetStringLibrary.Conv_IntToString` (`self.Table_Position`))))
    (:`then`
      (set `self.Paint Color` (`.Color_2_53DE62814B0B53C6911BB698D1B71F66` (break `/Game/Blueprints/Temporary/PaintType1_Canvas/STR_Colors` _returnvalue))))))

(event `self.ReceiveTick`
  (params (DeltaSeconds :type "Float (single-precision)"))
  (bind _returnvalue (`GameplayStatics.GetPlayerCameraManager` 0))
  (bind _returnvalue_2 (`PlayerCameraManager.GetCameraLocation` _returnvalue))
  (bind _outhits (`KismetSystemLibrary.LineTraceMulti` :`Start` _returnvalue_2 :`End` (+ _returnvalue_2 (* (`self.GetActorForwardVector` _returnvalue) 500.0)) :`TraceChannel` "TraceTypeQuery1" :`DrawDebugType` "ForOneFrame"))
  (for _array_element _outhits
    (bind (_bblockinghit _binitialoverlap _time _distance _location _impactpoint _normal _impactnormal _physmat _hitactor) (`GameplayStatics.BreakHitResult` _array_element))
    (bind _asbp_washable (cast `/Game/Blueprints/Temporary/PaintType2_PowerWash/BP_Washable` _hitactor))
    (`/Game/Blueprints/Temporary/PaintType2_PowerWash/BP_Washable.DrawToRenderTarget` _asbp_washable _impactpoint 500.0)
    (`KismetSystemLibrary.PrintString` "Hello")))

(event `Paint_Size_IncrementDown`
  ; Reduce paint radius
  (set `self.Paint_Radius` (- (`self.Paint_Radius`) (`self.Paint_Radius_Multiplier`))))

(event `Paint_Size_IncrementUp`
  ; Up paint radius
  (set `self.Paint_Radius` (+ (`self.Paint_Radius`) (`self.Paint_Radius_Multiplier`))))

(event `Paint_Color_Change`
  ; Change color
  (bind _result (`/Engine/EditorBlueprintResources/StandardMacros.IncrementInt` (`self.Table_Position`))
    (:`  `
      (bind _output_get (set `self.Table_Position` (mod _result 4)))
      ; Set color
      (bind _returnvalue (`|GetDataTableRow` (`self.DT_PaintColor`) (`KismetStringLibrary.Conv_StringToName` (`KismetStringLibrary.Conv_IntToString` _output_get)))
        (:`then`
          (set `self.Paint Color` (`.Color_2_53DE62814B0B53C6911BB698D1B71F66` (break `/Game/Blueprints/Temporary/PaintType1_Canvas/STR_Colors` _returnvalue))))))))

(fn `UserConstructionScript`)