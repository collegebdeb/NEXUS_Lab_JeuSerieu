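; BP_ParentCanvas is a paintable canvas that brush strokes are drawn onto at runtime.
; BeginPlay creates and clears a large render target, feeds it into a dynamic canvas material applied to every Canvas material slot, and creates a dynamic brush material.
; DrawBrush sets the brush texture and hue, then draws that material into the render target, centered on a normalized draw location scaled to the target's size.
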(event `self.ReceiveBeginPlay`
  (`|ExecutionSequence`
    (:`then_0`
      (bind _returnvalue (`KismetRenderingLibrary.CreateRenderTarget2D` 8192 8192 "RTF_RGBA16f" (struct)))
      (bind _output_get (set `self.RenderTarget` _returnvalue))
      (`KismetRenderingLibrary.ClearRenderTarget2D` _output_get (struct :`A` 0.547826)))
    (:`then_1`
      (bind _returnvalue_2 (`KismetMaterialLibrary.CreateDynamicMaterialInstance` "/Game/Blueprints/Temporary/Canvas_Mat.Canvas_Mat"))
      (for (_ _array_index) (`MeshComponent.GetMaterials` (`self.Canvas`))
        (`MaterialInstanceDynamic.SetTextureParameterValue` _returnvalue_2 "RenderTarget" (`self.RenderTarget`))
        (`PrimitiveComponent.SetMaterial` (`self.Canvas`) _array_index _returnvalue_2)))
    (:`then_2`
      (bind _returnvalue_3 (`KismetMaterialLibrary.CreateDynamicMaterialInstance` "/Game/Blueprints/Temporary/M_Brush.M_Brush"))
      (set `self.BrushMat` _returnvalue_3))))

(fn `DrawBrush`
  (params (BrushTexture :type "Texture2D Object Reference") (BrushSize :type "Float (double-precision)") (DrawLocation :type "Vector2D Structure") (BrushColor :type "LinearColor Structure"))
  (bind _brushmat (`self.BrushMat`))
  (bind _brushsize (`local.BrushSize`))
  (`|ExecutionSequence`
    (:`then_0`
      (`MaterialInstanceDynamic.SetTextureParameterValue` _brushmat "BrushTexture" BrushTexture)
      (`MaterialInstanceDynamic.SetVectorParameterValue` _brushmat "Hue" BrushColor))
    (:`then_1`
      (bind (_canvas _size _context) (`KismetRenderingLibrary.BeginDrawCanvasToRenderTarget` (`self.RenderTarget`)))
      (`Canvas.K2_DrawMaterial` _canvas (`self.BrushMat`) (- (* _size (`local.DrawLocation`)) (/ _brushsize 2.0)) (`KismetMathLibrary.MakeVector2D` _brushsize _brushsize) (0.0 0.0) (1.0 1.0) 0.0 (0.5 0.5))
      (`KismetRenderingLibrary.EndDrawCanvasToRenderTarget` _context))))

(fn `UserConstructionScript`)