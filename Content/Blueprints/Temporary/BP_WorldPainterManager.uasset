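; World painter manager that splats brush marks onto static mesh actors at a given hit UV.
; On an actor's first hit, every material slot gets a dynamic material and an R8 render target as BrushMask, all stamped using M_SplatBrush.
; The actor stores the targets through message calls.
; Later hits fetch them and use the collision face's SectionIndex to choose which target to draw into for each mesh component.
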(event `self.ReceiveBeginPlay`
  (`/Engine/EditorBlueprintResources/StandardMacros.Can Execute Cosmetic Events`
    (:`True`
      (bind _returnvalue (`KismetMaterialLibrary.CreateDynamicMaterialInstance` "/Game/Blueprints/Temporary/M_SplatBrush.M_SplatBrush"))
      (set `self.BrushMaterial` _returnvalue))))

(fn `PassPaintData`
  (params (IncomingActor :type "Actor Object Reference") (HitFaceIndex :type Integer) (HitUV :type "LinearColor Structure"))
  (locals (TempActorRenderTargets2D :type "Array of TextureRenderTarget2D Object Reference") (TemporaryActorStaticMesh :type "StaticMeshComponent Object Reference") (TemporaryMaterialSlot :type Integer) (TemporaryMaterialConstant :type "MaterialInterface Object Reference") (TemporaryMaterialDynamic :type "MaterialInstanceDynamic Object Reference") (TemporaryRenderTargets2D :type "TextureRenderTarget2D Object Reference"))
  (if (not (`KismetArrayLibrary.Array_Contains` (`self.PaintedActors`) (`local.IncomingActor`)))
    (`KismetArrayLibrary.Array_AddUnique` (`self.PaintedActors`) (`local.IncomingActor`))
    (for _array_element (`self.K2_GetComponentsByClass` (`local.IncomingActor`) "/Script/Engine.StaticMeshComponent")
      (bind _output_get (set `local.TemporaryActorStaticMesh` _array_element))
      (for (_array_element_2 _array_index) (`MeshComponent.GetMaterials` _output_get)
        (set `local.TemporaryMaterialConstant` _array_element_2)
        (set `local.TemporaryMaterialSlot` _array_index)
        (bind _returnvalue (`KismetMaterialLibrary.CreateDynamicMaterialInstance` (`local.TemporaryMaterialConstant`)))
        (set `local.TemporaryMaterialDynamic` _returnvalue)
        (`|ExecutionSequence`
          (:`then_0`
            (bind _returnvalue_2 (`KismetRenderingLibrary.CreateRenderTarget2D` 512 512 "RTF_R8"))
            (set `local.TemporaryRenderTargets2D` _returnvalue_2))
          (:`then_1`
            (`MaterialInstanceDynamic.SetTextureParameterValue` (`local.TemporaryMaterialDynamic`) "BrushMask" (`local.TemporaryRenderTargets2D`))
            (`PrimitiveComponent.SetMaterial` (`local.TemporaryActorStaticMesh`) (`local.TemporaryMaterialSlot`) (`local.TemporaryMaterialDynamic`))
            (`KismetArrayLibrary.Array_AddUnique` (`local.TempActorRenderTargets2D`) (`local.TemporaryRenderTargets2D`))
            (`|ExecutionSequence`
              (:`then_0`
                (`MaterialInstanceDynamic.SetVectorParameterValue` (`self.BrushMaterial`) "UV" (`local.HitUV`)))
              (:`then_1`
                (`KismetRenderingLibrary.DrawMaterialToRenderTarget` (`local.TemporaryRenderTargets2D`) (`self.BrushMaterial`))))))))
    (message `/Game/Blueprints/Temporary/BPI_Paintable.StorePaintedRTs` (`local.IncomingActor`) (`local.TempActorRenderTargets2D`))
    (else
      (bind _rendertarget2d (message `/Game/Blueprints/Temporary/BPI_Paintable.GetPaintedRTs` (`local.IncomingActor`)))
      (set `local.TempActorRenderTargets2D` _rendertarget2d)
      (for _array_element_3 (`self.K2_GetComponentsByClass` (`local.IncomingActor`) "/Script/Engine.StaticMeshComponent")
        (set `local.TemporaryActorStaticMesh` _array_element_3)
        (set `local.TemporaryRenderTargets2D` (`|GetArrayItem` (`local.TempActorRenderTargets2D`) (`PrimitiveComponent.GetMaterialFromCollisionFaceIndex` (`local.TemporaryActorStaticMesh`) (`local.HitFaceIndex`))))
        (`|ExecutionSequence`
          (:`then_0`
            (`MaterialInstanceDynamic.SetVectorParameterValue` (`self.BrushMaterial`) "UV" (`local.HitUV`)))
          (:`then_1`
            (`KismetRenderingLibrary.DrawMaterialToRenderTarget` (`local.TemporaryRenderTargets2D`) (`self.BrushMaterial`))))))))

(fn `UserConstructionScript`)