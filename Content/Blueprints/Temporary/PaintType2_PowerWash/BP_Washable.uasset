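; BP_Washable is a washable mesh actor that accumulates power-wash brush hits into a render-target mask.
; On BeginPlay, a scene capture renders the mesh with M_Unwrap into a texture, then restores its dynamic materials.
; DrawToRenderTarget feeds impact point and brush size to a brush material that reads that unwrap texture and draws into the hit mask.
; The mesh's layered materials read this mask as their OpacityMask blend parameter.
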(event `self.ReceiveBeginPlay`
  (bind _scenecapturecomponent2d (`self.SceneCaptureComponent2D`))
  (for _index (range (`PrimitiveComponent.GetNumMaterials` (`self.StaticMesh1`)))
    (bind _returnvalue (`PrimitiveComponent.CreateDynamicMaterialInstance` (`self.StaticMesh1`) _index (`self.Source_Material`) "None"))
    (`KismetArrayLibrary.Array_Add` (`self.Material_Instances`) _returnvalue))
  (`|ExecutionSequence`
    (:`then_0`
      (bind _returnvalue_2 (`KismetRenderingLibrary.CreateRenderTarget2D` 1024 1024))
      (bind _output_get (set `self.RT_Unwrap` _returnvalue_2))
      (set `SceneCaptureComponent2D.TextureTarget` _output_get _scenecapturecomponent2d)
      (`SceneCaptureComponent.ShowOnlyActorComponents` _scenecapturecomponent2d self false))
    (:`then_1`
      (bind _returnvalue_3 (`KismetRenderingLibrary.CreateRenderTarget2D` 1024 1024))
      (set `self.RT_Hit` _returnvalue_3)
      (for _array_element (`self.Material_Instances`)
        (`MaterialInstanceDynamic.SetTextureParameterValueByInfo` _array_element (make `MaterialParameterInfo` "OpacityMask" "BlendParameter" 0) (`self.RT_Hit`)))
      (`KismetRenderingLibrary.ClearRenderTarget2D` (`self.RT_Hit`)))
    (:`then_2`
      (`SceneComponent.K2_SetWorldRotation` (`self.SceneCaptureComponent2D`) (struct :`Pitch` -90.0 :`Yaw` -90.0) false false)
      (for _ (range (`PrimitiveComponent.GetNumMaterials` (`self.StaticMesh1`)))
        (`PrimitiveComponent.SetMaterial` (`self.StaticMesh1`) 0 "/Game/Blueprints/Temporary/PaintType2_PowerWash/M_Unwrap.M_Unwrap"))
      (`SceneCaptureComponent2D.CaptureScene` (`self.SceneCaptureComponent2D`))
      (for (_array_element_2 _array_index) (`self.Material_Instances`)
        (`PrimitiveComponent.SetMaterial` (`self.StaticMesh1`) _array_index _array_element_2))
      (bind _returnvalue_4 (`KismetMaterialLibrary.CreateDynamicMaterialInstance` "/Game/Blueprints/Temporary/PaintType2_PowerWash/MI_PowerWashable.MI_PowerWashable"))
      (bind _output_get_2 (set `self.MI_Brush` _returnvalue_4))
      (`MaterialInstanceDynamic.SetTextureParameterValue` _output_get_2 "Unwrapped" (`self.RT_Unwrap`)))))

(fn `DrawToRenderTarget`
  (params (ImpactPoint :type "Vector Structure") (BrushSize :type "Float (double-precision)"))
  (`MaterialInstanceDynamic.SetScalarParameterValue` (`self.MI_Brush`) "Size" BrushSize)
  (`MaterialInstanceDynamic.SetVectorParameterValue` (`self.MI_Brush`) "Position" (`KismetMathLibrary.Conv_VectorToLinearColor` (`local.ImpactPoint`)))
  (`KismetRenderingLibrary.DrawMaterialToRenderTarget` (`self.RT_Hit`) (`self.MI_Brush`)))

(fn `UserConstructionScript`
  (`StaticMeshComponent.SetStaticMesh` (`self.StaticMesh1`) (`self.Source_Mesh`)))