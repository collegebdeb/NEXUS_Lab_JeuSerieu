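; BP_Painter is a painter that calls PaintOnMesh every Tick with its current paint radius and color.
; On BeginPlay it loads the color from the DTPaintColor data table, using TablePosition as the row name.
; The Paint_Size events step the radius up or down, while Paint_Color_Change cycles through four table rows with a modulo.
; Both kinds of change print their new values as debug output.
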(event `self.ReceiveBeginPlay`
  (bind _returnvalue (`|GetDataTableRow` (`self.DT_PaintColor`) (`KismetStringLibrary.Conv_StringToName` (`KismetStringLibrary.Conv_IntToString` (`self.Table_Position`))))
    (:`then`
      (set `self.Paint Color` (`.Color_2_53DE62814B0B53C6911BB698D1B71F66` (break `/Game/Blueprints/Temporary/STR_Colors` _returnvalue))))))

(event `self.ReceiveTick`
  (params (DeltaSeconds :type "Float (single-precision)"))
  (`/Game/Blueprints/Temporary/BPFL_Utilities.PaintOnMesh` (`self.Paint_Radius`) (`self.Paint Color`)))

(event `Paint_Size_IncrementDown`
  (bind _output_get (set `self.Paint_Radius` (- (`self.Paint_Radius`) (`self.Paint_Radius_Multiplier`))))
  (`KismetSystemLibrary.PrintString` (`KismetStringLibrary.Concat_StrStr` "PaintRadius: " (`KismetStringLibrary.Conv_DoubleToString` _output_get))))

(event `Paint_Size_IncrementUp`
  (bind _output_get (set `self.Paint_Radius` (+ (`self.Paint_Radius`) (`self.Paint_Radius_Multiplier`))))
  (`KismetSystemLibrary.PrintString` (`KismetStringLibrary.Concat_StrStr` "PaintRadius: " (`KismetStringLibrary.Conv_DoubleToString` _output_get))))

(event `Paint_Color_Change`
  (bind _result (`/Engine/EditorBlueprintResources/StandardMacros.IncrementInt` (`self.Table_Position`))
    (:`  `
      (bind _output_get (set `self.Table_Position` (mod _result 4)))
      (bind _returnvalue (`|GetDataTableRow` (`self.DT_PaintColor`) (`KismetStringLibrary.Conv_StringToName` (`KismetStringLibrary.Conv_IntToString` _output_get)))
        (:`then`
          (bind _output_get_2 (set `self.Paint Color` (`.Color_2_53DE62814B0B53C6911BB698D1B71F66` (break `/Game/Blueprints/Temporary/STR_Colors` _returnvalue))))
          (`KismetSystemLibrary.PrintString` (`KismetStringLibrary.Conv_IntToString` (`self.Table_Position`)))
          (`KismetSystemLibrary.PrintString` (`KismetStringLibrary.Conv_ColorToString` _output_get_2)))))))

(fn `UserConstructionScript`)