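; BP_ButtonPath is an interactable button that moves BP_Dragon onto its next path and unlocks a linked door.
; On Interact, it checks CanInteract, then proceeds only if the level's dragon, found by class lookup, has completed its current path.
; It then deactivates itself, enables and disables the other actors in its two lists, and unlocks LinkedDoor, chaining progression between interactables.
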(event `/Game/Blueprints/LVL_Artiste3D/BlueprintActor/BPI_Interactable.Interact`
  (`self.CanInteract`
    (:`then`
      (`self.InteractButton`))
    (:`else`)))

(fn `InteractButton`
  (`self.CanInteract`
    (:`then`
      ; Start Movement
      (bind _returnvalue (`GameplayStatics.GetActorOfClass` "/Game/Blueprints/LVL_Artiste3D/BlueprintActor/BP_Dragon.BP_Dragon_C"))
      (if (>= (`/Game/Blueprints/LVL_Artiste3D/BlueprintActor/BP_Dragon.CompletionPercent` _returnvalue) 1.0)
        (`/Game/Blueprints/LVL_Artiste3D/BlueprintActor/BP_Dragon.SwitchToNextPath` _returnvalue)
        (`self.DeactivateButton`)
        (`|ExecutionSequence`
          (:`then_0`
            ; Set new interactibility
            (for _array_element (`self.SetInteractableOnPress`)
              (set `/Game/Blueprints/LVL_Artiste3D/BlueprintActor/BP_Button.CanInteract` true _array_element))
            (for _array_element_2 (`self.SetNotInteractableOnPress`)
              (`self.DeactivateButton` _array_element_2)))
          (:`then_1`
            (`/Game/Blueprints/LVL_Artiste3D/BlueprintActor/BP_SlidingDoor.UnlockDoor` (`|ConvertAsset` (`self.LinkedDoor`)))))))
    (:`else`)))

(fn `UserConstructionScript`
  (`parent.UserConstructionScript`))