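; Hologram bridge actor that materializes when OnEndOfLine is called and can later disappear once crossed by an overlap.
; Looping near-zero timers interpolate dynamic material parameters, fading opacity in, then driving IsHologram to zero and enabling collision.
; Once destroyable, overlapping DisableBridgeCollision either destroys it immediately or, with FadeOutBridge, reverts it to hologram and fades it before destruction.
; SpawnOtherDialogueTrigger keeps a referenced dialogue box's collision off until that overlap.
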(event `self.ReceiveBeginPlay`
  (bind _staticmesh (`self.StaticMesh`))
  (`|ExecutionSequence`
    (:`then_0`
      (if (`self.SpawnOtherDialogueTrigger?`)
        (bind _dialogueboxreference (`self.DialogueBoxReference`)
          (:`then`
            (`PrimitiveComponent.SetCollisionEnabled` (`/Game/Blueprints/SystemDialogue/Outdated/BP_DataAssetDialogueTriggerBox.Box` _dialogueboxreference) "NoCollision"))
          (:`else`))))
    (:`then_1`
      (bind _returnvalue (`PrimitiveComponent.CreateDynamicMaterialInstance` _staticmesh 0 (`PrimitiveComponent.GetMaterial` _staticmesh 0) "None"))
      (set `self.DynamicMaterial1` _returnvalue)
      (bind _returnvalue_2 (`PrimitiveComponent.CreateDynamicMaterialInstance` _staticmesh 1 (`PrimitiveComponent.GetMaterial` _staticmesh 1) "None"))
      (set `self.DynamicMaterial2` _returnvalue_2)
      (`PrimitiveComponent.SetCollisionEnabled` (`self.StaticMesh`) "NoCollision"))))

(event `FadeIn`
  (bind _returnvalue (`GameplayStatics.GetWorldDeltaSeconds`))
  (bind _dynamicmaterial1 (`self.DynamicMaterial1`))
  (bind _dynamicmaterial1_2 (`self.DynamicMaterial1`))
  (if (not (`self.IsFadingOut`))
    (bind _returnvalue_2 (`KismetMathLibrary.FInterpTo_Constant` (`self.CurrentInnerOpacity`) 0.5 _returnvalue (`self.InnerCapacityInterpSpeed`)))
    (set `self.CurrentInnerOpacity` _returnvalue_2)
    (bind _returnvalue_3 (`KismetMathLibrary.FInterpTo_Constant` (`self.CurrentOuterOpacity`) 10.0 _returnvalue (`self.OuterCapacityInterpSpeed`)))
    (set `self.CurrentOuterOpacity` _returnvalue_3)
    (`MaterialInstanceDynamic.SetScalarParameterValue` _dynamicmaterial1 "OpacityInner" (`self.CurrentInnerOpacity`))
    (`MaterialInstanceDynamic.SetScalarParameterValue` _dynamicmaterial1 "OpacityOuter" (`self.CurrentOuterOpacity`))
    (`MaterialInstanceDynamic.SetScalarParameterValue` _dynamicmaterial1_2 "OpacityInner" (`self.CurrentInnerOpacity`))
    (`MaterialInstanceDynamic.SetScalarParameterValue` _dynamicmaterial1_2 "OpacityOuter" (`self.CurrentOuterOpacity`))
    (if (and (== (`self.CurrentInnerOpacity`) 0.5) (== (`self.CurrentOuterOpacity`) 10.0))
      (`/Engine/EditorBlueprintResources/StandardMacros.DoOnce` false
        (:`Completed`
          (bind _returnvalue_4 (`KismetSystemLibrary.K2_SetTimerDelegate` (delegate `MaterialChange`) 1e-05 true true))
          (set `self.PBRFadeInTimer` _returnvalue_4)
          (`PrimitiveComponent.SetCollisionEnabled` (`self.StaticMesh`) "QueryAndPhysics"))))))

(event `MaterialChange`
  (if (not (`self.IsFadingOut`))
    (set `self.BridgeCanBeDestroyed?` true)
    (bind _returnvalue (`KismetMathLibrary.FInterpTo` (`self.CurrentSwitchValue`) 0.0 (`GameplayStatics.GetWorldDeltaSeconds`) (`self.SwitchValueInterpSpeed`)))
    (set `self.CurrentSwitchValue` _returnvalue)
    (`MaterialInstanceDynamic.SetScalarParameterValue` (`self.DynamicMaterial1`) "IsHologram" (`self.CurrentSwitchValue`))
    (`MaterialInstanceDynamic.SetScalarParameterValue` (`self.DynamicMaterial2`) "IsHologram" (`self.CurrentSwitchValue`))
    (`|ExecutionSequence`
      (:`then_0`
        (if (== (`self.CurrentSwitchValue`) 0.0)
          (`KismetSystemLibrary.K2_ClearAndInvalidateTimerHandle` (`self.FadeInTimer`))
          (`KismetSystemLibrary.K2_ClearAndInvalidateTimerHandle` (`self.PBRFadeInTimer`))))
      (:`then_1`
        (if (<= (`self.CurrentSwitchValue`) (`self.ValueBeforeCollisionEnable`))
          (`PrimitiveComponent.SetCollisionEnabled` (`self.StaticMesh`) "QueryAndPhysics"))))))

(event `/Game/Blueprints/SystemDialogue/Interfaces/BPI_EventCallAtEndOfLine.OnEndOfLine`
  (`SceneComponent.SetHiddenInGame` (`self.StaticMesh`) false false)
  (`|ExecutionSequence`
    (:`then_0`
      (`/Engine/EditorBlueprintResources/StandardMacros.DoOnce` false
        (:`Completed`
          (bind _returnvalue (`KismetSystemLibrary.K2_SetTimerDelegate` (delegate `FadeIn`) 1e-06 true true))
          (set `self.FadeInTimer` _returnvalue))))))

(event `FadeOut`
  (bind _returnvalue (`GameplayStatics.GetWorldDeltaSeconds`))
  (bind _dynamicmaterial1 (`self.DynamicMaterial1`))
  (bind _dynamicmaterial2 (`self.DynamicMaterial2`))
  (if (`self.IsFadingOut`)
    (`KismetSystemLibrary.PrintString` "fuckyoubitch")
    (`self.SetAllInterpSpeed`)
    (bind _returnvalue_2 (`KismetMathLibrary.FInterpTo_Constant` (`self.CurrentFadeOutInnerOpacity`) 0.0 _returnvalue (`self.FadeOutInnerOpacityInterpSpeed`)))
    (set `self.CurrentFadeOutInnerOpacity` _returnvalue_2)
    (bind _returnvalue_3 (`KismetMathLibrary.FInterpTo_Constant` (`self.CurrentFadeOutOuterCapacity`) 0.0 _returnvalue (`self.FadeOutOuterOpacityInterpSpeed`)))
    (set `self.CurrentFadeOutOuterCapacity` _returnvalue_3)
    (`MaterialInstanceDynamic.SetScalarParameterValue` _dynamicmaterial1 "OpacityInner" (`self.CurrentFadeOutInnerOpacity`))
    (`KismetSystemLibrary.PrintString` "mhmwhy" true true (struct :`G` 0.66 :`B` 1.0 :`A` 1.0) 0.0)
    (`MaterialInstanceDynamic.SetScalarParameterValue` _dynamicmaterial1 "OpacityOuter" (`self.CurrentFadeOutOuterCapacity`))
    (`MaterialInstanceDynamic.SetScalarParameterValue` _dynamicmaterial2 "OpacityInner" (`self.CurrentFadeOutInnerOpacity`))
    (`MaterialInstanceDynamic.SetScalarParameterValue` _dynamicmaterial2 "OpacityOuter" (`self.CurrentFadeOutOuterCapacity`))
    (if (and (<= (`self.CurrentFadeOutInnerOpacity`) 0.0) (<= (`self.CurrentFadeOutOuterCapacity`) 0.0))
      (`PrimitiveComponent.SetCollisionEnabled` (`self.StaticMesh`) "NoCollision")
      (`self.K2_DestroyActor`))))

(event `self.DisableBridgeCollision.OnComponentBeginOverlap`
  (params (OverlappedComponent :type "PrimitiveComponent Object Reference") (OtherActor :type "Actor Object Reference") (OtherComp :type "PrimitiveComponent Object Reference") (OtherBodyIndex :type Integer) (bFromSweep :type Boolean) (SweepResult :type "HitResult Structure (by ref)"))
  (bind _fadeoutbridge (`self.FadeOutBridge`))
  (if (`self.BridgeCanBeDestroyed?`)
    (if (`self.SpawnOtherDialogueTrigger?`)
      (if _fadeoutbridge :!label _label
        (bind _returnvalue (`KismetSystemLibrary.K2_SetTimerDelegate` (delegate `MaterialChangeFadeOut`) 1e-06 true true))
        (set `self.FadeOutTimer1` _returnvalue)
        (set `self.IsFadingOut` true)
        (if (`self.SpawnOtherDialogueTrigger?`)
          (`PrimitiveComponent.SetCollisionEnabled` (`/Game/Blueprints/SystemDialogue/Outdated/BP_DataAssetDialogueTriggerBox.Box` (`self.DialogueBoxReference`)) "QueryOnly"))
        (else
          (`PrimitiveComponent.SetCollisionEnabled` (`/Game/Blueprints/SystemDialogue/Outdated/BP_DataAssetDialogueTriggerBox.Box` (`self.DialogueBoxReference`)) "QueryOnly")
          (`self.K2_DestroyActor`)))
      (elif _fadeoutbridge
        (goto _label)
        (else
          (`self.K2_DestroyActor`))))))

(event `MaterialChangeFadeOut`
  (bind _returnvalue (`GameplayStatics.GetWorldDeltaSeconds`))
  (bind _dynamicmaterial1 (`self.DynamicMaterial1`))
  (bind _dynamicmaterial2 (`self.DynamicMaterial2`))
  (if (`self.IsFadingOut`)
    (set `self.FadeOutSwitchValueInterpSpeed` 0.5)
    (bind _returnvalue_2 (`KismetMathLibrary.FInterpTo_Constant` (`self.CurrentFadeOutSwitchValue`) 1.0 (`GameplayStatics.GetWorldDeltaSeconds`) (`self.FadeOutSwitchValueInterpSpeed`)))
    (set `self.CurrentFadeOutSwitchValue` _returnvalue_2)
    (`MaterialInstanceDynamic.SetScalarParameterValue` (`self.DynamicMaterial1`) "IsHologram" (`self.CurrentFadeOutSwitchValue`))
    (`MaterialInstanceDynamic.SetScalarParameterValue` (`self.DynamicMaterial2`) "IsHologram" (`self.CurrentFadeOutSwitchValue`))
    (if (== _returnvalue_2 1.0)
      (if (`self.IsFadingOut`)
        (`self.SetAllInterpSpeed`)
        (bind _returnvalue_3 (`KismetMathLibrary.FInterpTo_Constant` (`self.CurrentFadeOutInnerOpacity`) 0.0 _returnvalue (`self.FadeOutInnerOpacityInterpSpeed`)))
        (set `self.CurrentFadeOutInnerOpacity` _returnvalue_3)
        (bind _returnvalue_4 (`KismetMathLibrary.FInterpTo_Constant` (`self.CurrentFadeOutOuterCapacity`) 0.0 _returnvalue (`self.FadeOutOuterOpacityInterpSpeed`)))
        (set `self.CurrentFadeOutOuterCapacity` _returnvalue_4)
        (`MaterialInstanceDynamic.SetScalarParameterValue` _dynamicmaterial1 "OpacityInner" (`self.CurrentFadeOutInnerOpacity`))
        (`MaterialInstanceDynamic.SetScalarParameterValue` _dynamicmaterial1 "OpacityOuter" (`self.CurrentFadeOutOuterCapacity`))
        (`MaterialInstanceDynamic.SetScalarParameterValue` _dynamicmaterial2 "OpacityInner" (`self.CurrentFadeOutInnerOpacity`))
        (`MaterialInstanceDynamic.SetScalarParameterValue` _dynamicmaterial2 "OpacityOuter" (`self.CurrentFadeOutOuterCapacity`))
        (if (and (<= (`self.CurrentFadeOutInnerOpacity`) 0.0) (<= (`self.CurrentFadeOutOuterCapacity`) 0.0))
          (`PrimitiveComponent.SetCollisionEnabled` (`self.StaticMesh`) "NoCollision")
          (`self.K2_DestroyActor`))))))

(fn `SetAllInterpSpeed`
  (set `self.FadeOutInnerOpacityInterpSpeed` 4.0)
  (set `self.FadeOutOuterOpacityInterpSpeed` 4.0)
  (set `self.OuterCapacityInterpSpeed` 0.0)
  (set `self.InnerCapacityInterpSpeed` 0.0)
  (set `self.SwitchValueInterpSpeed` 0.0))

(fn `UserConstructionScript`
  (`StaticMeshComponent.SetStaticMesh` (`self.StaticMesh`) (`self.BrigdeMesh`)))