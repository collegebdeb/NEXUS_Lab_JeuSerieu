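; Hand bridge actor whose skeletal hand opens when the player comes within HandOpenDistance and closes when they move away.
; It starts with the close animation, then checks distance every Tick.
; Two DoOnce gates, each reset by the opposite action after a delay, alternate opening and closing, each with a sound.
; Opening scales animation rate and sound pitch with player speed, while closing plays at normal rate.
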(event `self.ReceiveBeginPlay`
  (`SkeletalMeshComponent.PlayAnimation` (`self.SkeletalMesh`) "/Game/Art/SkeletalMeshes/LowPolyHand/Animations/LowPolyHandAnimations_Cube_Anim_Armature_hand_close.LowPolyHandAnimations_Cube_Anim_Armature_hand_close" false))

(event `self.ReceiveTick`
  (params (DeltaSeconds :type "Float (single-precision)"))
  (bind _skeletalmesh (`self.SkeletalMesh`))
  (bind _sc_mainouverture (`self.SC_MainOuverture`))
  (bind _sc_mainouverture_2 (`self.SC_MainOuverture`))
  (bind _skeletalmesh_2 (`self.SkeletalMesh`))
  (bind _returnvalue (`KismetMathLibrary.MapRangeClamped` (`self.GetPlayerSpeed`) 550.0 900.0 1.0 2.0))
  (bind _returnvalue_2 (`SkeletalMeshComponent.IsPlaying` (`self.SkeletalMesh`)))
  (if (not (<= (`self.GetDistanceTo` (`GameplayStatics.GetPlayerPawn` 0)) (`self.HandOpenDistance`)))
    (`/Engine/EditorBlueprintResources/StandardMacros.DoOnce` false :!label _label
      (:`Completed`
        (if (not _returnvalue_2)
          (set `SkeletalMeshComponent.GlobalAnimRateScale` 1.0 _skeletalmesh)
          (`SkeletalMeshComponent.PlayAnimation` _skeletalmesh "/Game/Art/SkeletalMeshes/LowPolyHand/Animations/LowPolyHandAnimations_Cube_Anim_Armature_hand_close.LowPolyHandAnimations_Cube_Anim_Armature_hand_close" false)
          (set `self.InRange` false)
          ; joue le son de main
          (set `AudioComponent.PitchMultiplier` 1.0 _sc_mainouverture_2)
          (`AudioComponent.Play` _sc_mainouverture_2 0.0)
          (`KismetSystemLibrary.Delay` 1.0)
          (goto _label_2 :!via `Reset`))))
    (else
      (`/Engine/EditorBlueprintResources/StandardMacros.DoOnce` false :!label _label_2
        (:`Completed`
          (if (not (and _returnvalue_2 (`self.InRange`)))
            (set `SkeletalMeshComponent.GlobalAnimRateScale` _returnvalue _skeletalmesh_2)
            (`SkeletalMeshComponent.PlayAnimation` _skeletalmesh_2 "/Game/Art/SkeletalMeshes/LowPolyHand/Animations/LowPolyHand_Opening_Anim_Armature_hand_open.LowPolyHand_Opening_Anim_Armature_hand_open" false)
            (set `self.InRange` true)
            (set `AudioComponent.PitchMultiplier` _returnvalue _sc_mainouverture)
            (`AudioComponent.Play` _sc_mainouverture 0.0)
            (`KismetSystemLibrary.Delay` 2.0)
            (goto _label :!via `Reset`)))))))

(fn `UserConstructionScript`)