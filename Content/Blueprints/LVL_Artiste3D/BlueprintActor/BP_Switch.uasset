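; Interactable light switch that, when used inside its trigger, turns on a list of point lights one after another.
; Lights start dark, then Tick compares Unix timestamps to restore each intensity at a fixed interval.
; After the last light, it plays an optional level sequence and signals linked BPI_Interactable actors.
; Dialogues run at press, after lighting and after the sequence, with optional player movement lock until the lights finish.
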(event `/Game/Blueprints/LVL_ConcepteurDeNiveau/Interfaces/BPI_InteractInfo.StartInteraction`
  ; Activation
  (if (`self.CanInteract?`)
    (`GameplayStatics.PlaySound2D` "/Engine/VREditor/Sounds/UI/Flashlight_Switch.Flashlight_Switch" 1.0 1.0 0.0 null null)
    (`|ExecutionSequence`
      (:`then_0`
        ; One Time Event
        (if (not (`self.IsLightOn`))
          (set `self.IsLightOn` true)
          (`KismetSystemLibrary.PrintString` "Turn light on")
          (set `self.CanWidgetBeVisible?` false)
          (`self.HideWidget`)))
      (:`then_1`
        (set `self.TimeActivated` (`KismetMathLibrary.ToUnixTimestampDouble` (`KismetMathLibrary.UtcNow`)))
        (`|ExecutionSequence`
          (:`then_0`
            (`self.RunDialogues` (`self.DialoguesAtButtonPress`)))
          (:`then_1`
            (`self.LockMovementsOnPress`
              (:`then`
                (set `/Game/FirstPerson/Blueprints/BP_FirstPersonCharacter.CanMove?` false (cast `/Game/FirstPerson/Blueprints/BP_FirstPersonCharacter` (`GameplayStatics.GetPlayerPawn` 0) :!pure true)))
              (:`else`))))))
    (else
      (`self.HideWidget`))))

(event `self.ReceiveBeginPlay`
  (`SceneComponent.SetVisibility` (`self.Widget`) false false)
  ; Lights Off
  (for _array_element (`self.LightInfo`)
    (bind _pointlightref (break `/Game/Blueprints/LVL_Artiste3D/Structures/S_Lights` _array_element))
    (`/Engine/EditorBlueprintResources/StandardMacros.IsValid` _pointlightref
      (:`Is Valid`
        (bind _lightcomponent (`Light.LightComponent` _pointlightref)
          (:`then`
            (`LightComponent.SetIntensity` _lightcomponent 0.0))
          (:`else`))))))

(event `self.ReceiveTick`
  (params (DeltaSeconds :type "Float (single-precision)"))
  (bind _lightinfo (`self.LightInfo`))
  ; Light Sequence
  (if (!= 0.0 (`self.TimeActivated`))
    (for (_array_element _array_index) _lightinfo
      (if (< (+ (* (`KismetMathLibrary.Conv_IntToDouble` _array_index) (`self.LightsActivationInterval`)) (`self.TimeActivated`)) (`KismetMathLibrary.ToUnixTimestampDouble` (`KismetMathLibrary.UtcNow`)))
        (bind (_pointlightref _pointlightintensity) (break `/Game/Blueprints/LVL_Artiste3D/Structures/S_Lights` _array_element))
        (`/Engine/EditorBlueprintResources/StandardMacros.IsValid` _pointlightref
          (:`Is Valid`
            (bind _lightcomponent (`Light.LightComponent` _pointlightref)
              (:`then`
                (`LightComponent.SetIntensity` _lightcomponent _pointlightintensity)
                (if (== (+ _array_index 1) (`KismetArrayLibrary.Array_Length` _lightinfo))
                  (set `self.TimeActivated` 0.0)
                  (`KismetSystemLibrary.Delay` 1.0)
                  (`|ExecutionSequence`
                    (:`then_0`
                      (bind _sequencetoplay (`self.SequenceToPlay`)
                        (:`then`
                          (bind _sequenceplayer (`LevelSequenceActor.SequencePlayer` _sequencetoplay)
                            (:`then`
                              (`MovieSceneSequencePlayer.Play` _sequenceplayer))
                            (:`else`)))
                        (:`else`)))
                    (:`then_1`
                      (`self.LockMovementsOnPress`
                        (:`then`
                          (set `/Game/FirstPerson/Blueprints/BP_FirstPersonCharacter.CanMove?` true (cast `/Game/FirstPerson/Blueprints/BP_FirstPersonCharacter` (`GameplayStatics.GetPlayerPawn` 0) :!pure true)))
                        (:`else`
                          _))
                      (`KismetSystemLibrary.Delay` 1.0)
                      (`|ExecutionSequence`
                        (:`then_0`
                          (`self.RunDialogues` (`self.DialoguesAfterButtonPress`)))
                        (:`then_1`
                          (`KismetSystemLibrary.Delay` (+ 1.0 (`TimeManagementBlueprintLibrary.Conv_QualifiedFrameTimeToSeconds` (`MovieSceneSequencePlayer.GetDuration` _sequenceplayer))))
                          (`self.RunDialogues` (`self.DialoguesAfterLevelSequence`)))))
                    (:`then_2`
                      (for _array_element_2 (`self.EnableAfterActivation`)
                        (bind _asbpi_interactable (cast `/Game/Blueprints/LVL_Artiste3D/BlueprintActor/BPI_Interactable` (`|ConvertAsset` _array_element_2)))
                        (`/Game/Blueprints/LVL_Artiste3D/BlueprintActor/BPI_Interactable.InteractScalar` _asbpi_interactable 67.0))))))
              (:`else`))))))))

(event `self.Trigger.OnComponentBeginOverlap`
  (params (OverlappedComponent :type "PrimitiveComponent Object Reference") (OtherActor :type "Actor Object Reference") (OtherComp :type "PrimitiveComponent Object Reference") (OtherBodyIndex :type Integer) (bFromSweep :type Boolean) (SweepResult :type "HitResult Structure (by ref)"))
  ; Widget Control
  (set `self.CanInteract?` true)
  (if (`self.CanWidgetBeVisible?`)
    (`SceneComponent.SetVisibility` (`self.Widget`) true false)))

(event `self.Trigger.OnComponentEndOverlap`
  (params (OverlappedComponent :type "PrimitiveComponent Object Reference") (OtherActor :type "Actor Object Reference") (OtherComp :type "PrimitiveComponent Object Reference") (OtherBodyIndex :type Integer))
  ; Widget Control
  (set `self.CanInteract?` false)
  (`SceneComponent.SetVisibility` (`self.Widget`) false false :!label _label))

(event `HideWidget`
  ; Widget Control
  (goto _label))

(fn `UserConstructionScript`)