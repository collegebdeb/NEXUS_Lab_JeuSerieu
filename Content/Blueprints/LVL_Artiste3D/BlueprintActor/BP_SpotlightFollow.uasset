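; BP_SpotlightFollow is a spotlight actor that keeps itself aimed at the BP_Dragon actor in the level.
; BeginPlay waits one tick, then caches the dragon found with GetActorOfClass.
; Tick turns the whole actor toward the dragon's location each frame with a look-at rotation, without checking that the reference is valid.
; A time-based HSV rainbow color effect for the light remains in the graph but is disconnected.
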(event `self.ReceiveBeginPlay`
  (`parent.ReceiveBeginPlay`)
  (`KismetSystemLibrary.DelayUntilNextTick`)
  (bind _returnvalue (`GameplayStatics.GetActorOfClass` "/Game/Blueprints/LVL_Artiste3D/BlueprintActor/BP_Dragon.BP_Dragon_C"))
  (set `self.Dragon` _returnvalue))

(event `self.ReceiveTick`
  (params (DeltaSeconds :type "Float (single-precision)"))
  (`parent.ReceiveTick` DeltaSeconds)
  (`self.K2_SetActorRotation` (`KismetMathLibrary.FindLookAtRotation` (`self.K2_GetActorLocation`) (`self.K2_GetActorLocation` (`self.Dragon`)))))

(fn `UserConstructionScript`
  (`parent.UserConstructionScript`))