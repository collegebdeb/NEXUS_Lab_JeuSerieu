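; BP_DragonRoar is an actor that travels in a continuous loop along the spline of a referenced Path.
; Each Tick derives completion from UTC Unix time modulo LoopDuration, so position follows the wall clock rather than accumulated delta time.
; It applies the spline's world-space location with sweep and its local-space rotation.
; An invalid Path prints an error with the actor's name.
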(event `self.ReceiveTick`
  (params (DeltaSeconds :type "Float (single-precision)"))
  (bind _path (`self.Path`))
  (bind _loopduration (`self.LoopDuration`))
  (bind _spline (`/Game/Blueprints/LVL_Artiste3D/BlueprintActor/BP_Path.Spline` _path))
  (bind _returnvalue (`KismetMathLibrary.Lerp` 0.0 (`SplineComponent.GetSplineLength` _spline) (/ (mod (`KismetMathLibrary.ToUnixTimestampDouble` (`KismetMathLibrary.UtcNow`)) _loopduration) _loopduration)))
  (`/Engine/EditorBlueprintResources/StandardMacros.IsValid` _path
    (:`Is Valid`
      (`self.K2_SetActorLocation` (`SplineComponent.GetLocationAtDistanceAlongSpline` _spline _returnvalue "World") true)
      (`self.K2_SetActorRotation` (`SplineComponent.GetRotationAtDistanceAlongSpline` _spline _returnvalue "Local")))
    (:`Is Not Valid`
      ; Error
      (`KismetSystemLibrary.PrintString` (`KismetStringLibrary.Concat_StrStr` (`KismetSystemLibrary.GetDisplayName` self) " PATH INVALID") true true (struct :`R` 1.0 :`A` 1.0) 0.0))))

(fn `UserConstructionScript`)