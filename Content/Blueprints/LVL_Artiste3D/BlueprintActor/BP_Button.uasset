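; BP_Button is an interactable button that triggers a linked actor and plays dialogue when pressed.
; Interact plays a sound, calls Interact on the linked actor through BPI_Interactable, then runs the player's UI dialogue indexed by press count.
; When IsReusable is valid, BP_Dragon's movement-completed event re-enables interaction.
; Separate functions disable the button and hide its widget, or enable the next stage's button.
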(event `self.ReceiveBeginPlay`
  (bind _returnvalue (`GameplayStatics.GetActorOfClass` "/Game/Blueprints/LVL_Artiste3D/BlueprintActor/BP_Dragon.BP_Dragon_C"))
  (bind _output_get (set `self.DragonObject` _returnvalue))
  (`self.IsReusable`
    (:`then`
      (add `/Game/Blueprints/LVL_Artiste3D/BlueprintActor/BP_Dragon.DragonMovementCompleted` _output_get (delegate `SetCanInteract`)))
    (:`else`)))

(event `SetCanInteract`
  (set `self.CanInteract` true))

(event `/Game/Blueprints/LVL_Artiste3D/BlueprintActor/BPI_Interactable.Interact`
  (`self.InteractButton`))

(fn `ActivateNextStageButton`
  (bind _nextstagebutton (`self.NextStageButton`)
    (:`then`
      (`self.SetCanInteract` (`|ConvertAsset` _nextstagebutton)))
    (:`else`)))

(fn `DeactivateButton`
  (set `self.CanInteract` false)
  (`SceneComponent.SetHiddenInGame` (`self.Widget`) true false))

(fn `InteractButton`
  (`GameplayStatics.PlaySoundAtLocation` (`self.InteractionSound`) (`self.K2_GetActorLocation`) (struct) (`self.Volume Multiplier`) (`self.Pitch Multiplier`) (`self.Start Time`) null null null null)
  (`|ExecutionSequence`
    (:`then_0`
      (bind _callinteractonactor (`self.CallInteractOnActor`)
        (:`then`
          (bind _asbpi_interactable (cast `/Game/Blueprints/LVL_Artiste3D/BlueprintActor/BPI_Interactable` (`|ConvertAsset` _callinteractonactor)))
          (`/Game/Blueprints/LVL_Artiste3D/BlueprintActor/BPI_Interactable.Interact` _asbpi_interactable))
        (:`else`)))
    (:`then_1`
      (bind _result (`/Engine/EditorBlueprintResources/StandardMacros.IncrementInt` (`self.NumberOfTimePressed`))
        (:`  `
          (bind _output_rowhandles (break `/Game/Blueprints/LVL_Artiste3D/Structures/S_RowHandleArray` (`|GetArrayItem` (`self.DialoguesArray`) (- _result 1))))
          (`/Game/UI/Widgets/WBP_DialogueBox.RunDialogue` (`/Game/FirstPerson/Blueprints/BP_FirstPersonCharacter.UIDialogue` (cast `/Game/FirstPerson/Blueprints/BP_FirstPersonCharacter` (`GameplayStatics.GetPlayerPawn` 0) :!pure true)) _output_rowhandles true)
          (`KismetSystemLibrary.PrintString` "Button pressed"))))))

(fn `UserConstructionScript`)