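; BP_Pointer is an animated pointer actor whose Fleche (arrow) component bobs up and down while spinning around its vertical axis.
; Each Tick, a sine wave scaled by BobbingSpeed is remapped between MinHeight and MaxHeight for relative Z, while RotationSpeed drives a wrapped yaw.
; Both motions derive directly from the UTC wall-clock timestamp, not from game time or accumulated delta time.
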(event `self.ReceiveTick`
  (params (DeltaSeconds :type "Float (single-precision)"))
  (bind _returnvalue (`KismetMathLibrary.ToUnixTimestampDouble` (`KismetMathLibrary.UtcNow`)))
  (`SceneComponent.K2_SetRelativeLocationAndRotation` (`self.fleche`) (`KismetMathLibrary.MakeVector` 0.0 0.0 (`KismetMathLibrary.MapRangeClamped` (`KismetMathLibrary.Sin` (* (`KismetMathLibrary.MultiplyByPi` _returnvalue) (`self.BobbingSpeed`))) -1.0 1.0 (`self.MinHeight`) (`self.MaxHeight`))) (`KismetMathLibrary.MakeRotator` 0.0 0.0 (mod (* _returnvalue (`self.RotationSpeed`)) 360.0)) false false))

(fn `UserConstructionScript`)