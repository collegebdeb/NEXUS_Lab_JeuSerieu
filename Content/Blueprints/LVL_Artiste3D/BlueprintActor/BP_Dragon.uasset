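; Dragon actor that travels along a list of spline paths and changes color through toggleable RGB channels.
; Tick advances completion at constant speed scaled by spline length, moving the actor with sweep and optionally rotating it along the path.
; At path end it stops and calls DragonMovementCompleted; SwitchToNextPath starts the next spline.
; A dynamic material on the cube mixes the enabled channels, showing graybox gray when all are off.
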(event `self.ReceiveBeginPlay`
  (`self.UpdateMaterial` false))

(event `self.ReceiveTick`
  (params (DeltaSeconds :type "Float (single-precision)"))
  (bind _currentpath (`self.CurrentPath`))
  (bind _spline (`/Game/Blueprints/LVL_Artiste3D/BlueprintActor/BP_Path.Spline` _currentpath))
  (bind _returnvalue (`SplineComponent.GetSplineLength` _spline))
  (`self.IsMoving`
    (:`then`
      (if (> (`KismetArrayLibrary.Array_Length` (`self.Paths`)) 0)
        (`/Engine/EditorBlueprintResources/StandardMacros.IsValid` _currentpath
          (:`Is Valid`
            ;[0.7473 0.7812 0 0.5] Compute location and rotation
            (bind _output_get (`self.UpdateCompletionPercent` DeltaSeconds _returnvalue))
            (bind _returnvalue_2 (`KismetMathLibrary.Lerp` 0.0 _returnvalue _output_get))
            (`self.K2_SetActorLocation` (`SplineComponent.GetLocationAtDistanceAlongSpline` _spline _returnvalue_2 "World") true)
            (`self.RotateWithPath`
              (:`then`
                (`self.K2_SetActorRotation` (`SplineComponent.GetRotationAtDistanceAlongSpline` _spline _returnvalue_2 "Local")))
              (:`else`
                _))
            ;[0.15 1 0.15 0.5] Stop the movement
            (if (>= (`self.CompletionPercent`) 1.0)
              (set `self.IsMoving` false)
              (`self.DragonMovementCompleted`)))
          (:`Is Not Valid`
            ;[0.15 0 0 0.5] Error handling
            ;; Error current path
            (`KismetSystemLibrary.PrintString` (`KismetStringLibrary.Concat_StrStr` (`KismetSystemLibrary.GetDisplayName` self) " PATH INVALID") true true (struct :`R` 1.0 :`A` 1.0) 0.0)))
        (else
          ;; Error path list
          (`KismetSystemLibrary.PrintString` (`KismetStringLibrary.Concat_StrStr` (`KismetSystemLibrary.GetDisplayName` self) "NO VALID PATH") true true (struct :`R` 1.0 :`A` 1.0) 0.0))))
    (:`else`)))

(fn `SwitchToNextPath`
  (bind _result (`/Engine/EditorBlueprintResources/StandardMacros.IncrementInt` (`self.CurrentPathIndex`))
    (:`  `
      (set `self.CurrentPath` (`|GetArrayItem` (`self.Paths`) _result))
      (set `self.IsMoving` true) ; Start moving
      (set `self.CompletionPercent` 0.0) ; Go to start of path
    )))

(fn `ToggleColorChannel`
  (params (Channel :type "/Game/Blueprints/LVL_Artiste3D/Data/Enumeration/E_ColorsRGB Enum" :default "NewEnumerator0"))
  (returns (red :type Boolean) (green :type Boolean) (blue :type Boolean))
  (bind _color (`self.Color`))
  (bind _color_2 (`self.Color`))
  ; Toggle
  (`BlueprintMapLibrary.Map_Add` _color Channel (not (`BlueprintMapLibrary.Map_Find` _color Channel)))
  (return (`.Value` (`BlueprintMapLibrary.Map_GetKeyValueByIndex` _color_2)) (`.Value` (`BlueprintMapLibrary.Map_GetKeyValueByIndex` _color_2 1)) (`.Value` (`BlueprintMapLibrary.Map_GetKeyValueByIndex` _color_2 2))))

(fn `UpdateCompletionPercent`
  (params (DeltaTime :type "Float (single-precision)") (SplineLentgth :type "Float (double-precision)"))
  (returns (Output_Get :type "Float (double-precision)"))
  (bind _output_get (set `self.CompletionPercent` (+ (`self.CompletionPercent`) (/ (* DeltaTime (`self.MovementSpeed`) 100.0) SplineLentgth))))
  (return _output_get))

(fn `UpdateMaterial`
  (params (red :type Boolean) (green :type Boolean) (blue :type Boolean))
  (locals (Material :type "MaterialInstanceDynamic Object Reference"))
  ; Dynamic material
  (bind _returnvalue (`KismetMaterialLibrary.CreateDynamicMaterialInstance` (`self.DragonMaterial`)))
  (bind _output_get (set `local.Material` _returnvalue))
  (if (or red green blue)
    ; Update color
    (`MaterialInstanceDynamic.SetVectorParameterValue` _output_get "Albedo" (make `LinearColor` (`KismetMathLibrary.Conv_BoolToDouble` red) (`KismetMathLibrary.Conv_BoolToDouble` green) (`KismetMathLibrary.Conv_BoolToDouble` blue) 1.0))
    (else
      (`MaterialInstanceDynamic.SetVectorParameterValue` _output_get "Albedo" (struct :`R` 0.2 :`G` 0.2 :`B` 0.2 :`A` 1.0)) ; Graybox look
    ))
  (`PrimitiveComponent.SetMaterial` (`self.Cube`) 0 _output_get))

(fn `UserConstructionScript`)