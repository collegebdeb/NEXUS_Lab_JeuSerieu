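; BP_Cage is a cage actor that spirals vertically to a height received through InteractScalar, with mechanical loop and end sounds.
; That event restarts the CageAnimation timeline at a distance-based play rate, and Tick lerps height from it, deriving yaw from height times a multiplier.
; If a BP_EmergencySpotLights actor exists, BeginPlay stores its offset and hides the Dragon component, and timeline updates move the lights with the cage.
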(event `self.ReceiveBeginPlay`
  (bind (_returnvalue_x _returnvalue_y _returnvalue_z) (`KismetMathLibrary.BreakVector` (`self.K2_GetActorLocation`)))
  (bind _output_get (set `self.TargetHeight` _returnvalue_z))
  (set `self.HeightAtBeginRise` _output_get)
  (bind _returnvalue (`GameplayStatics.GetActorOfClass` "/Game/Blueprints/LVL_Artiste3D/BlueprintActor/BP_EmergencySpotLights.BP_EmergencySpotLights_C"))
  (bind _output_get_2 (set `self.EmergencyLights` _returnvalue))
  (`/Engine/EditorBlueprintResources/StandardMacros.IsValid` _output_get_2
    (:`Is Valid`
      (set `self.EmergencyLightsOffset` (- (`self.K2_GetActorLocation` _returnvalue) (`self.K2_GetActorLocation`)))
      (`SceneComponent.SetVisibility` (`self.Dragon`) false false))))

(event `self.ReceiveTick`
  (params (DeltaSeconds :type "Float (single-precision)"))
  (bind (_returnvalue_x _returnvalue_y _returnvalue_z) (`KismetMathLibrary.BreakVector` (`self.K2_GetActorLocation`)))
  (bind _returnvalue (`KismetMathLibrary.Lerp` (`self.HeightAtBeginRise`) (`self.TargetHeight`) (stale `/Game/Blueprints/LVL_Artiste3D/BlueprintActor/BPI_Interactable.InteractScalar` _animation)))
  (`self.K2_SetActorLocationAndRotation` (`KismetMathLibrary.MakeVector` _returnvalue_x _returnvalue_y _returnvalue) (`KismetMathLibrary.MakeRotator` 0.0 0.0 (* _returnvalue (`self.RotationMultiplier`)))))

(event `/Game/Blueprints/LVL_Artiste3D/BlueprintActor/BPI_Interactable.InteractScalar`
  (params (Value :type "Float (double-precision)"))
  (bind (_returnvalue_roll _returnvalue_pitch _returnvalue_yaw) (`KismetMathLibrary.BreakRotator` (`self.K2_GetActorRotation`)))
  (bind (_returnvalue_x _returnvalue_y _returnvalue_z) (`KismetMathLibrary.BreakVector` (`self.K2_GetActorLocation`)))
  (bind _relativelocation (`SceneComponent.RelativeLocation` (`self.Cage`)))
  (set `self.TargetHeight` Value)
  (`TimelineComponent.SetPlayRate` (`self.CageAnimation`) (/ (- (`self.TargetHeight`) (`self.HeightAtBeginRise`)) (/ 1.0 (`self.RisingSpeed`)) 10000.0))
  (set `self.HeightAtBeginRise` _returnvalue_z)
  (bind (_direction _animation) (`Timeline|CageAnimation` :!via `PlayFromStart`)
    (:`Update`
      ; son de la cage
      (`KismetSystemLibrary.Delay` 1.0)
      (`GameplayStatics.PlaySoundAtLocation` "/Game/Audio/SallePrincipale/CageMécanique/SC_CageMécaniqueLoop.SC_CageMécaniqueLoop" _relativelocation (struct) 1.0 1.0 0.0 null null null null)
      (bind _emergencylights (`self.EmergencyLights`)
        (:`then`
          (bind (_returnvalue_roll_2 _returnvalue_pitch_2 _returnvalue_yaw_2) (`KismetMathLibrary.BreakRotator` (`self.K2_GetActorRotation` _emergencylights)))
          (set `self.EmergencyLightsRotationOffset` (- _returnvalue_yaw_2 _returnvalue_yaw))
          (`self.K2_SetActorLocationAndRotation` _emergencylights (+ (`self.K2_GetActorLocation`) (`self.EmergencyLightsOffset`)) (`KismetMathLibrary.MakeRotator` 0.0 0.0 (+ (* (`KismetMathLibrary.Lerp` (`self.HeightAtBeginRise`) (`self.TargetHeight`) _animation) (`self.RotationMultiplier`)) (`self.EmergencyLightsRotationOffset`))) false false))
        (:`else`)))
    (:`Finished`
      (`KismetSystemLibrary.Delay` 3.0)
      (`GameplayStatics.PlaySoundAtLocation` "/Game/Audio/SallePrincipale/CageMécanique/SC_CageMécaniqueFin.SC_CageMécaniqueFin" _relativelocation (struct) 1.0 1.0 0.0 null null null null))))

(fn `UserConstructionScript`)