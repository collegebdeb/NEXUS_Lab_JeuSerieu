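; BP_Paraplegic is a one-shot trigger that temporarily paralyses the player on overlap and steers their view to a set rotation.
; The first overlap disables movement and locks the view on BP_FirstPersonCharacter, then records a UTC timestamp.
; While paralysed, Tick eases the camera toward TargetPlayerRotation through Aim, scaled by ViewControlSpeed and delta time.
; Once DurationOfParalysis has elapsed in wall-clock time, Tick restores movement and view control.
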(event `self.ReceiveActorBeginOverlap`
  (params (OtherActor :type "Actor Object Reference"))
  (bind _returnvalue (`GameplayStatics.GetPlayerPawn` 0))
  (bind _asbp_first_person_character (cast `/Game/FirstPerson/Blueprints/BP_FirstPersonCharacter` _returnvalue :!pure true))
  (if (== OtherActor _returnvalue)
    (`/Engine/EditorBlueprintResources/StandardMacros.DoOnce` false
      (:`Completed`
        (set `self.ParalizedTime` (`KismetMathLibrary.ToUnixTimestampDouble` (`KismetMathLibrary.UtcNow`)))
        (set `/Game/FirstPerson/Blueprints/BP_FirstPersonCharacter.CanMove?` false _asbp_first_person_character)
        (set `/Game/FirstPerson/Blueprints/BP_FirstPersonCharacter.LockView` true _asbp_first_person_character)
        (set `self.IsParaplegic` true)))))

(event `self.ReceiveTick`
  (params (DeltaSeconds :type "Float (single-precision)"))
  (bind (_targetplayerrotation_roll _targetplayerrotation_pitch _targetplayerrotation_yaw) (`KismetMathLibrary.BreakRotator` (`self.TargetPlayerRotation`)))
  (bind _asbp_first_person_character (cast `/Game/FirstPerson/Blueprints/BP_FirstPersonCharacter` (`GameplayStatics.GetPlayerPawn` 0) :!pure true))
  (bind _returnvalue (* (`self.ViewControlSpeed`) DeltaSeconds))
  (bind (_returnvalue_roll _returnvalue_pitch _returnvalue_yaw) (`KismetMathLibrary.BreakRotator` (`SceneComponent.K2_GetComponentRotation` (`/Game/FirstPerson/Blueprints/BP_FirstPersonCharacter.FirstPersonCamera` _asbp_first_person_character))))
  (`self.IsParaplegic`
    (:`then`
      ; Force the player to look at the target rotation
      (`/Game/FirstPerson/Blueprints/BP_FirstPersonCharacter.Aim` _asbp_first_person_character (* (- _targetplayerrotation_yaw _returnvalue_yaw) _returnvalue) (* (- _returnvalue_pitch _targetplayerrotation_pitch) _returnvalue))
      (`/Game/FirstPerson/Blueprints/BP_FirstPersonCharacter.Aim` _asbp_first_person_character (* (- _targetplayerrotation_yaw _returnvalue_yaw) _returnvalue) (* (- _returnvalue_pitch _targetplayerrotation_pitch) _returnvalue))
      (if (> (`KismetMathLibrary.ToUnixTimestampDouble` (`KismetMathLibrary.UtcNow`)) (+ (`self.ParalizedTime`) (`self.DurationOfParalysis`)))
        (set `/Game/FirstPerson/Blueprints/BP_FirstPersonCharacter.CanMove?` true _asbp_first_person_character)
        (set `/Game/FirstPerson/Blueprints/BP_FirstPersonCharacter.LockView` false _asbp_first_person_character)
        (set `self.IsParaplegic` false)))
    (:`else`)))

(fn `UserConstructionScript`)