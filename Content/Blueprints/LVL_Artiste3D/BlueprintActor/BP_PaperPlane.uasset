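; BP_PaperPlane is an actor that flies continuously along the spline of a referenced Path actor.
; Each Tick, UpdateCompletionPercent advances progress by MovementSpeed scaled to spline length, keeping speed independent of path length.
; The progress wraps modulo 1 to loop, setting a swept world-space location and a rotation sampled in spline local space.
; An invalid Path prints an error with the actor's name.
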(event `self.ReceiveTick`
  (params (DeltaSeconds :type "Float (single-precision)"))
  (bind _path (`self.Path`))
  (bind _spline (`/Game/Blueprints/LVL_Artiste3D/BlueprintActor/BP_Path.Spline` _path))
  (bind _returnvalue (`SplineComponent.GetSplineLength` _spline))
  (`/Engine/EditorBlueprintResources/StandardMacros.IsValid` _path
    (:`Is Valid`
      ;[0.7473 0.7812 0 0.5] Compute location and rotation
      (bind _output_get (`self.UpdateCompletionPercent` DeltaSeconds _returnvalue))
      (bind _returnvalue_2 (`KismetMathLibrary.Lerp` 0.0 _returnvalue (mod _output_get 1.0)))
      (`self.K2_SetActorLocation` (`SplineComponent.GetLocationAtDistanceAlongSpline` _spline _returnvalue_2 "World") true)
      (`self.K2_SetActorRotation` (`SplineComponent.GetRotationAtDistanceAlongSpline` _spline _returnvalue_2 "Local")))
    (:`Is Not Valid`
      ; Error current path
      (`KismetSystemLibrary.PrintString` (`KismetStringLibrary.Concat_StrStr` (`KismetSystemLibrary.GetDisplayName` self) " PATH INVALID") true true (struct :`R` 1.0 :`A` 1.0) 0.0))))

(fn `UpdateCompletionPercent`
  (params (DeltaTime :type "Float (single-precision)") (SplineLentgth :type "Float (double-precision)"))
  (returns (Output_Get :type "Float (double-precision)"))
  (bind _output_get (set `self.CompletionPercent` (+ (`self.CompletionPercent`) (/ (* DeltaTime (`self.MovementSpeed`) 100.0) SplineLentgth))))
  (return _output_get))

(fn `UserConstructionScript`)