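; BP_ButtonAnimation is an interactable button that previews a good or bad animation on a dragon object.
; Interact, gated by CanInteract, calls InteractButton, which plays the looping good or bad animation on the dragon's FinalMesh according to IsGoodAnimation.
; A good pick deactivates every animation button in the level and calls ActivateNextStageButton inside that loop.
; A bad pick deactivates only this button.
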(event `/Game/Blueprints/LVL_Artiste3D/BlueprintActor/BPI_Interactable.Interact`
  (`self.CanInteract`
    (:`then`
      (`self.InteractButton`))
    (:`else`)))

(fn `InteractButton`
  (bind _dragonobject (`self.DragonObject`))
  (bind _finalmesh (`/Game/Blueprints/LVL_Artiste3D/BlueprintActor/BP_Dragon.FinalMesh` _dragonobject))
  (`self.IsGoodAnimation`
    (:`then`
      (`SkeletalMeshComponent.PlayAnimation` _finalmesh (`/Game/Blueprints/LVL_Artiste3D/BlueprintActor/BP_Dragon.GoodAnimation` _dragonobject) true)
      ; Deactivate animation buttons
      (bind _outactors (`GameplayStatics.GetAllActorsOfClass` "BP_ButtonAnimation_C"))
      (for _array_element _outactors
        (`self.DeactivateButton` _array_element)
        (`self.ActivateNextStageButton`)))
    (:`else`
      (`SkeletalMeshComponent.PlayAnimation` _finalmesh (`/Game/Blueprints/LVL_Artiste3D/BlueprintActor/BP_Dragon.BadAnimation` _dragonobject) true)
      (`self.DeactivateButton`))))

(fn `UserConstructionScript`
  (`parent.UserConstructionScript`))