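; BP_BaphometGang is a flock manager that spawns BP_Baphomet members at its location and moves them as boids.
; Each tick, Separation and Cohesion build a steering vector per member in the Members map, then members turn gradually toward it and move forward.
; Separation also avoids other gangs' members and, when those exist, the player pawn.
; Cohesion effectively pulls toward the gang actor rather than the flock average, and Alignement is unused.
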(event `self.ReceiveBeginPlay`
  (`/Engine/EditorBlueprintResources/StandardMacros.DoOnce` false
    (:`Completed`
      (for _ (range 1 (+ (`self.NumberOfMember`) 1))
        (bind _returnvalue (`|SpawnActorFromClass` "/Game/Blueprints/LVL_Artiste3D/BlueprintActor/BP_Baphomet.BP_Baphomet_C" (`KismetMathLibrary.MakeTransform` (+ (`self.K2_GetActorLocation`) (* (`KismetMathLibrary.RandomUnitVector`) 1.0)) (`KismetMathLibrary.RandomRotator` false)) "Undefined" "MultiplyWithRoot" null null))
        (`BlueprintMapLibrary.Map_Add` (`self.Members`) _returnvalue)))))

(event `self.ReceiveTick`
  (params (DeltaSeconds :type "Float (single-precision)"))
  (bind _members (`self.Members`))
  (`parent.ReceiveTick` DeltaSeconds)
  (`self.Debug`
    (:`then`
      (`KismetSystemLibrary.DrawDebugSphere` (`self.K2_GetActorLocation`) 10.0 12 (struct :`R` 1.0 :`G` 1.0 :`A` 1.0) 0.0 1.0))
    (:`else`
      _))
  (bind _keypin (`|MapForEach` _members)
    (:`then`
      (`self.Separation` _keypin DeltaSeconds)
      (`self.Cohesion` _keypin DeltaSeconds))
    (:`CompletedPin`
      (bind (_keypin_2 _valuepin) (`|MapForEach` _members)
        (:`then`
          (bind _returnvalue (`self.K2_GetActorLocation` _keypin_2))
          (bind _returnvalue_2 (`KismetMathLibrary.FindLookAtRotation` (0.0 0.0 0.0) (`KismetMathLibrary.VLerp` (`self.GetActorForwardVector` _keypin_2) (`KismetMathLibrary.GetForwardVector` (`KismetMathLibrary.FindLookAtRotation` _returnvalue (+ _returnvalue (* _valuepin DeltaSeconds)))) (`KismetMathLibrary.FClamp` (* DeltaSeconds (`self.TurningSpeed`))))))
          (`self.K2_SetActorRotation` _keypin_2 _returnvalue_2 false)
          (`self.K2_SetActorLocation` _keypin_2 (+ _returnvalue (* (`KismetMathLibrary.GetForwardVector` _returnvalue_2) (`self.speed`))) false false))
        (:`CompletedPin`
          (set `self.FlockLocation` (0.0 0.0 0.0)))))))

(fn `Alignement`
  (params (CurrentMember :type "Actor Object Reference") (DeltaTime :type "Float (double-precision)"))
  (locals (AverageForwardVector :type "Vector Structure"))
  (bind _members (`self.Members`))
  (bind _othermembers (`self.GetAllMemberButCurrentMember` CurrentMember))
  (for _array_element _othermembers
    (set `local.AverageForwardVector` (+ (`local.AverageForwardVector`) (`self.GetActorForwardVector` _array_element))))
  (bind _output_get (set `local.AverageForwardVector` (/ (`local.AverageForwardVector`) (`KismetArrayLibrary.Array_Length` _othermembers))))
  (`BlueprintMapLibrary.Map_Add` _members CurrentMember (+ (`BlueprintMapLibrary.Map_Find` _members CurrentMember) (+ (`self.K2_GetActorLocation` CurrentMember) (`KismetMathLibrary.VLerp` (`self.GetActorForwardVector` CurrentMember) _output_get (* (`self.AlignementFactor`) DeltaTime))))))

(fn `Cohesion`
  (params (CurrentMember :type "Actor Object Reference") (DeltaTime :type "Float (double-precision)"))
  (locals (AverageLocation :type "Vector Structure"))
  (bind _returnvalue (`self.K2_GetActorLocation` CurrentMember))
  (bind _returnvalue_2 (`self.K2_GetActorLocation`))
  (bind _members (`self.Members`))
  (bind _othermembers (`self.GetAllMemberButCurrentMember` CurrentMember))
  (for _array_element _othermembers
    (set `local.AverageLocation` (+ (`local.AverageLocation`) _returnvalue_2 _returnvalue_2)))
  (bind _output_get (set `local.AverageLocation` (/ (`local.AverageLocation`) (* (`KismetArrayLibrary.Array_Length` _othermembers) 2)))) ; Real average location
  (`self.Debug`
    (:`then`
      (`KismetSystemLibrary.DrawDebugSphere` _output_get 30.0 12 (struct :`R` 1.0 :`G` 1.0 :`A` 1.0)))
    (:`else`
      _))
  (bind _returnvalue_3 (- _output_get _returnvalue))
  (`BlueprintMapLibrary.Map_Add` _members CurrentMember (+ (`BlueprintMapLibrary.Map_Find` _members CurrentMember) (* _returnvalue_3 (`self.CohesionFactor`))))
  (`self.Debug`
    (:`then`
      (`KismetSystemLibrary.DrawDebugArrow` _returnvalue (+ _returnvalue _returnvalue_3) 1.0 (struct :`R` 1.0 :`G` 1.0 :`A` 1.0) 0.0 1.0))
    (:`else`)))

(fn `GetAllButCurrentMember`
  (params (CurrentMember :type "Actor Object Reference"))
  (returns (OtherMembers :type "Array of Actor Object Reference"))
  (locals (Others :type "Array of Actor Object Reference") (NewLocalVar :type "Vector Structure" :default (0.0 0.0 0.0)))
  (bind _keypin (`|MapForEach` (`self.Members`))
    (:`then`
      (if (!= _keypin CurrentMember)
        (`KismetArrayLibrary.Array_Add` (`local.Others`) _keypin)))
    (:`CompletedPin`
      (bind _outactors (`GameplayStatics.GetAllActorsOfClass` "BP_BaphometGang_C"))
      (for _array_element _outactors
        (if (!= _array_element self)
          (bind _keypin_2 (`|MapForEach` (`/Game/Blueprints/LVL_Artiste3D/BlueprintActor/BP_BaphometGang.Members` _array_element))
            (:`then`
              (bind _returnvalue (`KismetArrayLibrary.Array_Add` (`local.Others`) _keypin_2))
              (if true
                (`KismetArrayLibrary.Array_Add` (`local.Others`) (`GameplayStatics.GetPlayerPawn` 0)))))))
      (return (`local.Others`)))))

(fn `GetAllMemberButCurrentMember`
  (params (CurrentMember :type "Actor Object Reference"))
  (returns (OtherMembers :type "Array of Actor Object Reference"))
  (locals (Others :type "Array of Actor Object Reference"))
  (bind _keypin (`|MapForEach` (`self.Members`))
    (:`then`
      (if (!= _keypin CurrentMember)
        (`KismetArrayLibrary.Array_Add` (`local.Others`) _keypin)))
    (:`CompletedPin`
      (return (`local.Others`)))))

(fn `Separation`
  (params (CurrentMember :type "Actor Object Reference") (DeltaTime :type "Float (double-precision)"))
  (locals (SeparationVector :type "Vector Structure"))
  (bind _returnvalue (`self.K2_GetActorLocation` CurrentMember))
  (bind _returnvalue_2 (`self.K2_GetActorLocation` CurrentMember))
  (bind _separationvector (`local.SeparationVector`))
  (bind _othermembers (`self.GetAllButCurrentMember` CurrentMember))
  (for _array_element _othermembers
    (bind _returnvalue_3 (- (`self.K2_GetActorLocation` _array_element) _returnvalue_2))
    (bind _returnvalue_4 (* (`KismetMathLibrary.Normal` _returnvalue_3) (/ (`self.SeparationFactor`) (`KismetMathLibrary.VSize` _returnvalue_3)) -100.0))
    (set `local.SeparationVector` (+ (`local.SeparationVector`) _returnvalue_4))
    (`self.Debug`
      (:`then`
        (`KismetSystemLibrary.DrawDebugArrow` _returnvalue_2 (+ (/ _returnvalue_4 1) _returnvalue_2) 1.0 (struct :`R` 1.0 :`A` 1.0) 0.0 10.0))
      (:`else`)))
  (for _ _othermembers
    _)
  (`BlueprintMapLibrary.Map_Add` (`self.Members`) CurrentMember _separationvector)
  (`self.Debug`
    (:`then`
      (`KismetSystemLibrary.DrawDebugArrow` _returnvalue (+ _returnvalue (/ _separationvector 1)) 1.0 (struct :`B` 1.0 :`A` 1.0) 0.0 10.0))
    (:`else`)))

(fn `UserConstructionScript`)