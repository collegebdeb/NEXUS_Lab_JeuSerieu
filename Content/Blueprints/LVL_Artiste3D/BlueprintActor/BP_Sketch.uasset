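; BP_Sketch is an interactable sketch in the Artiste3D level that the player inspects to unlock a linked door.
; Interact calls InteractButton, which sets the door openable, freezes the first-person character, flags it as inspecting and shows a WBP_Inspect widget stored on that character.
; It then deactivates its button, activates the next stage's button, and hides and destroys itself.
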(event `/Game/Blueprints/LVL_Artiste3D/BlueprintActor/BPI_Interactable.Interact`
  (`self.InteractButton`))

(fn `InteractButton`
  (set `/Game/Blueprints/LVL_Artiste3D/BlueprintActor/BP_SlidingDoor.CanBeOpened` true (`|ConvertAsset` (`self.LinkedDoor`)))
  (bind _returnvalue (`GameplayStatics.GetActorOfClass` "/Game/FirstPerson/Blueprints/BP_FirstPersonCharacter.BP_FirstPersonCharacter_C"))
  (set `/Game/FirstPerson/Blueprints/BP_FirstPersonCharacter.CanMove?` false _returnvalue)
  (set `/Game/FirstPerson/Blueprints/BP_FirstPersonCharacter.InspectingSketch` true _returnvalue)
  (bind _returnvalue_2 (`|CreateWidget` "/Game/UI/Widgets/WBP_Inspect.WBP_Inspect_C"))
  (bind _output_get (set `/Game/FirstPerson/Blueprints/BP_FirstPersonCharacter.InspectionWidget` _returnvalue_2 _returnvalue))
  (`UserWidget.AddToViewport` _output_get 0)
  (`self.DeactivateButton`)
  (`self.ActivateNextStageButton`)
  (`self.SetActorHiddenInGame` true)
  (`self.K2_DestroyActor`))

(fn `UserConstructionScript`
  (`parent.UserConstructionScript`))