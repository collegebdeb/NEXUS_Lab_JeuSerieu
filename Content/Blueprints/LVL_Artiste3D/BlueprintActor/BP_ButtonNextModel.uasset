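; BP_ButtonNextModel is an interactable button in the Artiste3D level that advances a dragon object to its next model.
; On Interact, it checks that CanInteract is valid, then calls NextModel on DragonObject.
; When that call returns true, the button deactivates itself and activates the next stage button.
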(event `/Game/Blueprints/LVL_Artiste3D/BlueprintActor/BPI_Interactable.Interact`
  (`self.CanInteract`
    (:`then`
      (`self.InteractButton`))
    (:`else`)))

(fn `InteractButton`
  (bind _isfinalmesh (`/Game/Blueprints/LVL_Artiste3D/BlueprintActor/BP_Dragon.NextModel` (`self.DragonObject`)))
  (if _isfinalmesh
    (`self.DeactivateButton`)
    (`self.ActivateNextStageButton`)))

(fn `UserConstructionScript`
  (`parent.UserConstructionScript`))