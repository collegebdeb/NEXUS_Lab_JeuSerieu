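; Trigger actor that starts the final portal cutscene when the first-person character enters its box, firing only once.
; On overlap it creates and plays the PortalBaking level sequence, then moves the BP_PortalSpline2 actor to a hardcoded location.
; It then sets HasTriggerPortal and loops the separate PortalSequence indefinitely.
; Disconnected leftover nodes hold unused ping-pong playback, pause and delay logic.
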(event `self.ReceiveBeginPlay`)

(event `self.ReceiveActorBeginOverlap`
  (params (OtherActor :type "Actor Object Reference")))

(event `self.ReceiveTick`
  (params (DeltaSeconds :type "Float (single-precision)")))

(event `self.Box.OnComponentBeginOverlap`
  (params (OverlappedComponent :type "PrimitiveComponent Object Reference") (OtherActor :type "Actor Object Reference") (OtherComp :type "PrimitiveComponent Object Reference") (OtherBodyIndex :type Integer) (bFromSweep :type Boolean) (SweepResult :type "HitResult Structure (by ref)"))
  (cast `/Game/FirstPerson/Blueprints/BP_FirstPersonCharacter` OtherActor)
  (`/Engine/EditorBlueprintResources/StandardMacros.DoOnce` false
    (:`Completed`
      (bind _outactor (`LevelSequencePlayer.CreateLevelSequencePlayer` "/Game/Levels/VFX_Baking/PortalBaking.PortalBaking"))
      (`MovieSceneSequencePlayer.Play` (`LevelSequenceActor.SequencePlayer` _outactor))
      (bind _returnvalue (`GameplayStatics.GetActorOfClass` "/Game/Art/Niagara/BP_PortalSpline2.BP_PortalSpline2_C"))
      (`self.K2_SetActorLocation` _returnvalue (-80.0 -2140.0 4850.0) false false)
      (set `self.HasTriggerPortal` true)
      (`MovieSceneSequencePlayer.PlayLooping` (`LevelSequenceActor.SequencePlayer` (`self.PortalSequence`)) -1))))

(fn `UserConstructionScript`)