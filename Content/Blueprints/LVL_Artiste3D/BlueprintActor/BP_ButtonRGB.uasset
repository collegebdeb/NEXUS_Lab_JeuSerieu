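; Interactable RGB button that raises or lowers one color channel of a target actor by a set increment.
; Each press updates that actor's clamped color in a map on GM_FirstPerson, recolors it, then calls a color update and activates the next stage button.
; Recoloring squares each channel to adjust the color scale and sets Albedo on component materials, creating dynamic M_DragonTexture instances where none exist.
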(event `self.ReceiveBeginPlay`
  (`parent.ReceiveBeginPlay`))

(event `/Game/Blueprints/LVL_Artiste3D/BlueprintActor/BPI_Interactable.Interact`
  (`self.CanInteract`
    (:`then`
      (`self.InteractButton`))
    (:`else`)))

(fn `InteractButton`
  (`parent.InteractButton`)
  (bind _colorvalues (`self.UpdateColorValues`))
  (`self.UpdateMaterial` _colorvalues)
  (`self.UpdateColorValue`)
  (`self.ActivateNextStageButton`))

(fn `UpdateColorValues`
  (returns (ColorValues :type "/Game/Blueprints/LVL_Artiste3D/Data/S_RGBValues Structure"))
  (locals (GameMode :type "/Game/FirstPerson/Blueprints/GM_FirstPerson Object Reference"))
  (bind _objectcolorvalues (`/Game/FirstPerson/Blueprints/GM_FirstPerson.ObjectColorValues` (`local.GameMode`)))
  (bind _returnvalue (* (select `/Game/Blueprints/LVL_Artiste3D/Data/Enumeration/E_DeIncrease` (`self.Action`) :`NewEnumerator1` -1 :`NewEnumerator0` 1) (`self.IncrementColorValue`)))
  (`|ExecutionSequence`
    (:`then_0`
      (bind _output_get (set `local.GameMode` (cast `/Game/FirstPerson/Blueprints/GM_FirstPerson` (`GameplayStatics.GetGameMode`) :!pure true))))
    (:`then_1`
      (bind (_value _returnvalue_2) (`BlueprintMapLibrary.Map_Find` (`/Game/FirstPerson/Blueprints/GM_FirstPerson.ObjectColorValues` _output_get) (`self.ActorToColor`)))
      (if (not _returnvalue_2)
        ; Create values
        (`BlueprintMapLibrary.Map_Add` (`/Game/FirstPerson/Blueprints/GM_FirstPerson.ObjectColorValues` (`local.GameMode`)) (`self.ActorToColor`) (make `/Game/Blueprints/LVL_Artiste3D/Data/S_RGBValues` 0.0)))
      ; Update values
      (switch `/Game/Blueprints/LVL_Artiste3D/Data/Enumeration/E_ColorsRGB` (`self.Color`)
        (:`NewEnumerator2`
          (bind (_red _green _blue) (break `/Game/Blueprints/LVL_Artiste3D/Data/S_RGBValues` _value))
          (`BlueprintMapLibrary.Map_Add` _objectcolorvalues (`self.ActorToColor`) (make `/Game/Blueprints/LVL_Artiste3D/Data/S_RGBValues` _red _green (`KismetMathLibrary.FClamp` (+ _blue _returnvalue)))))
        (:`NewEnumerator1`
          (bind (_red_2 _green_2 _blue_2) (break `/Game/Blueprints/LVL_Artiste3D/Data/S_RGBValues` _value))
          (`BlueprintMapLibrary.Map_Add` _objectcolorvalues (`self.ActorToColor`) (make `/Game/Blueprints/LVL_Artiste3D/Data/S_RGBValues` _red_2 (`KismetMathLibrary.FClamp` (+ _green_2 _returnvalue)) _blue_2)))
        (:`NewEnumerator0`
          (bind (_red_3 _green_3 _blue_3) (break `/Game/Blueprints/LVL_Artiste3D/Data/S_RGBValues` _value))
          (`BlueprintMapLibrary.Map_Add` _objectcolorvalues (`self.ActorToColor`) (make `/Game/Blueprints/LVL_Artiste3D/Data/S_RGBValues` (`KismetMathLibrary.FClamp` (+ _returnvalue _red_3)) _green_3 _blue_3)))))
    (:`then_2`
      (return (`BlueprintMapLibrary.Map_Find` (`/Game/FirstPerson/Blueprints/GM_FirstPerson.ObjectColorValues` (`local.GameMode`)) (`self.ActorToColor`))))))

(fn `UpdateMaterial`
  (params (ColorValues :type "/Game/Blueprints/LVL_Artiste3D/Data/S_RGBValues Structure"))
  (locals (ColorValuesVar :type "/Game/Blueprints/LVL_Artiste3D/Data/S_RGBValues Structure") (PrimitiveComponentToColor :type "PrimitiveComponent Object Reference"))
  (bind (_colorvaluesvar_red _colorvaluesvar_green _colorvaluesvar_blue) (break `/Game/Blueprints/LVL_Artiste3D/Data/S_RGBValues` (`local.ColorValuesVar`)))
  (bind (_colorvaluesvar_red_2 _colorvaluesvar_green_2 _colorvaluesvar_blue_2) (break `/Game/Blueprints/LVL_Artiste3D/Data/S_RGBValues` (`local.ColorValuesVar`)))
  (set `local.ColorValuesVar` (make `/Game/Blueprints/LVL_Artiste3D/Data/S_RGBValues` (`KismetMathLibrary.Square` ColorValues_red_6_C7004B9F48D7BB6E845CA4A631B2B438) (`KismetMathLibrary.Square` ColorValues_green_7_BACDE01541AC4B80C2DA478BE95A0D1F) (`KismetMathLibrary.Square` ColorValues_blue_8_896F655F44E4F4CBB1B6EEA66BEBAD11))) ; no spaghetti code
  ; Get the material to color
  (for _array_element (`self.K2_GetComponentsByClass` (`|ConvertAsset` (`self.ActorToColor`)) "/Script/Engine.ActorComponent")
    (bind _output_get (set `local.PrimitiveComponentToColor` (cast `PrimitiveComponent` _array_element :!pure true)))
    (for _index (range (+ (`KismetMathLibrary.SelectInt` (`PrimitiveComponent.GetNumMaterials` _output_get) 0 (`self.RecolorAllMat`)) 1))
      (bind _asmaterial_instance_dynamic (cast `MaterialInstanceDynamic` (`PrimitiveComponent.GetMaterial` (`local.PrimitiveComponentToColor`) _index))
        (:`then`
          ; Apply new color
          (`MaterialInstanceDynamic.SetVectorParameterValue` _asmaterial_instance_dynamic "Albedo" (make `LinearColor` _colorvaluesvar_red _colorvaluesvar_green _colorvaluesvar_blue)))
        (:`CastFailed`
          ; Create dynamic material if none
          (bind _returnvalue (`KismetMaterialLibrary.CreateDynamicMaterialInstance` "/Game/Blueprints/LVL_Artiste3D/M_DragonTexture.M_DragonTexture"))
          (`MaterialInstanceDynamic.SetVectorParameterValue` _returnvalue "Albedo" (make `LinearColor` _colorvaluesvar_red_2 _colorvaluesvar_green_2 _colorvaluesvar_blue_2))
          (`PrimitiveComponent.SetMaterial` (`local.PrimitiveComponentToColor`) _index _returnvalue))))))

(fn `UserConstructionScript`
  (`parent.UserConstructionScript`))