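; BP_ColorWallTrigger is a trigger actor that transitions the material of assigned walls once the player pawn overlaps it.
; After the overlap sets a flag, Tick raises TransitionValue from 0 toward 1 over TransitionDuration.
; Each tick, it calls CreateDynamicMaterialInstance on the first material slot of each wall's retrieved primitive component and writes the TransitionValue scalar parameter.
; The flag is never reset, so updates continue after completion.
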(event `self.ReceiveActorBeginOverlap`
  (params (OtherActor :type "Actor Object Reference"))
  ; On trigger enter -> transition
  (if (== OtherActor (`GameplayStatics.GetPlayerPawn` 0))
    (set `self.DoTransition` true)))

(event `self.ReceiveTick`
  (params (DeltaSeconds :type "Float (single-precision)"))
  ; Update the transition value
  (`self.DoTransition`
    (:`then`
      (set `self.TransitionValue` (`KismetMathLibrary.FClamp` (+ (`self.TransitionValue`) (/ DeltaSeconds (`self.TransitionDuration`)))))
      ; For every wall to change
      (for _array_element (`self.Walls`)
        (bind _asprimitive_component (cast `PrimitiveComponent` (`self.GetComponentByClass` (`|ConvertAsset` _array_element) "/Script/Engine.ActorComponent")))
        ; Make the material editable
        (bind _returnvalue (`PrimitiveComponent.CreateDynamicMaterialInstance` _asprimitive_component 0 (`PrimitiveComponent.GetMaterial` _asprimitive_component 0) "None"))
        ; Apply transition state
        (`MaterialInstanceDynamic.SetScalarParameterValue` _returnvalue "TransitionValue" (`self.TransitionValue`))))
    (:`else`)))

(fn `UserConstructionScript`)