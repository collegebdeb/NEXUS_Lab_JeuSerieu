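; BP_ColorButtons is a control panel pairing decrease and increase buttons for one RGB channel of a target actor.
; On BeginPlay it passes channel, target, step, action and dialogues to both child BP_ButtonRGB actors.
; It binds their color update event to refresh a percentage text read from GM_FirstPerson's ObjectColorValues map.
; Activate enables interaction on both buttons, and Deactivate calls DeactivateButton on each.
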(event `self.ReceiveBeginPlay`
  (bind _incrementcolorvalue (`self.IncrementColorValue`))
  (bind _colorchannel (`self.ColorChannel`))
  (bind _actortocolor (`self.ActorToColor`))
  (bind _asbp_button_rgb (cast `/Game/Blueprints/LVL_Artiste3D/BlueprintActor/BP_ButtonRGB` (`ChildActorComponent.ChildActor` (`self.BP_ButtonRGB_Decrease`)) :!pure true))
  (bind _asbp_button_rgb_2 (cast `/Game/Blueprints/LVL_Artiste3D/BlueprintActor/BP_ButtonRGB` (`ChildActorComponent.ChildActor` (`self.BP_ButtonRGB_Increase`)) :!pure true))
  (bind (_red _green _blue) (break `/Game/Blueprints/LVL_Artiste3D/Data/S_RGBValues` (`BlueprintMapLibrary.Map_Find` (`/Game/FirstPerson/Blueprints/GM_FirstPerson.ObjectColorValues` (cast `/Game/FirstPerson/Blueprints/GM_FirstPerson` (`GameplayStatics.GetGameMode`) :!pure true)) (`self.ActorToColor`))))
  (`|ExecutionSequence`
    (:`then_0`
      ; Set variables of the buttons BP
      (set `/Game/Blueprints/LVL_Artiste3D/BlueprintActor/BP_ButtonRGB.Color` _colorchannel _asbp_button_rgb)
      (set `/Game/Blueprints/LVL_Artiste3D/BlueprintActor/BP_ButtonRGB.ActorToColor` _actortocolor _asbp_button_rgb)
      (set `/Game/Blueprints/LVL_Artiste3D/BlueprintActor/BP_ButtonRGB.IncrementColorValue` _incrementcolorvalue _asbp_button_rgb)
      (set `/Game/Blueprints/LVL_Artiste3D/BlueprintActor/BP_ButtonRGB.Action` "NewEnumerator1" _asbp_button_rgb)
      (set `/Game/Blueprints/LVL_Artiste3D/BlueprintActor/BP_Button.DialoguesArray` (`self.DecreaseButtonDialoguesArray`) _asbp_button_rgb))
    (:`then_1`
      (set `/Game/Blueprints/LVL_Artiste3D/BlueprintActor/BP_ButtonRGB.Color` _colorchannel _asbp_button_rgb_2)
      (set `/Game/Blueprints/LVL_Artiste3D/BlueprintActor/BP_ButtonRGB.ActorToColor` _actortocolor _asbp_button_rgb_2)
      (set `/Game/Blueprints/LVL_Artiste3D/BlueprintActor/BP_ButtonRGB.IncrementColorValue` _incrementcolorvalue _asbp_button_rgb_2)
      (set `/Game/Blueprints/LVL_Artiste3D/BlueprintActor/BP_ButtonRGB.Action` "NewEnumerator0" _asbp_button_rgb_2)
      (set `/Game/Blueprints/LVL_Artiste3D/BlueprintActor/BP_Button.DialoguesArray` (`self.IncreaseButtonDialoguesArray`) _asbp_button_rgb_2))
    (:`then_2`
      (add `/Game/Blueprints/LVL_Artiste3D/BlueprintActor/BP_ButtonRGB.UpdateColorValue` _asbp_button_rgb (delegate `UpdateColorText`))
      (add `/Game/Blueprints/LVL_Artiste3D/BlueprintActor/BP_ButtonRGB.UpdateColorValue` _asbp_button_rgb_2 (delegate `UpdateColorText`)))
    (:`then_3`
      ; Update text value
      (`TextRenderComponent.K2_SetText` (`self.ColorValue`) (`KismetTextLibrary.Conv_StringToText` (`KismetStringLibrary.Concat_StrStr` (`KismetStringLibrary.Conv_DoubleToString` (* (select `/Game/Blueprints/LVL_Artiste3D/Data/Enumeration/E_ColorsRGB` (`self.ColorChannel`) :`NewEnumerator2` _blue :`NewEnumerator1` _green :`NewEnumerator0` _red) 100.0)) "%")) :!label _label))
    (:`then_4`
      (bind _asbp_button_rgb_3 (cast `/Game/Blueprints/LVL_Artiste3D/BlueprintActor/BP_ButtonRGB` (`self.GetParentActor`)))
      (set `/Game/Blueprints/LVL_Artiste3D/BlueprintActor/BP_Button.InteractionSound` "/Game/Audio/SonAppuyerBouton/SC_BoutonAppuyeAigu.SC_BoutonAppuyeAigu" _asbp_button_rgb_3))))

(event `UpdateColorText`
  ; Update text value
  (goto _label))

(fn `Activate`
  (set `/Game/Blueprints/LVL_Artiste3D/BlueprintActor/BP_Button.CanInteract` true (cast `/Game/Blueprints/LVL_Artiste3D/BlueprintActor/BP_ButtonRGB` (`ChildActorComponent.ChildActor` (`self.BP_ButtonRGB_Decrease`)) :!pure true))
  (set `/Game/Blueprints/LVL_Artiste3D/BlueprintActor/BP_Button.CanInteract` true (cast `/Game/Blueprints/LVL_Artiste3D/BlueprintActor/BP_ButtonRGB` (`ChildActorComponent.ChildActor` (`self.BP_ButtonRGB_Increase`)) :!pure true)))

(fn `Deactivate`
  (`/Game/Blueprints/LVL_Artiste3D/BlueprintActor/BP_Button.DeactivateButton` (cast `/Game/Blueprints/LVL_Artiste3D/BlueprintActor/BP_ButtonRGB` (`ChildActorComponent.ChildActor` (`self.BP_ButtonRGB_Decrease`)) :!pure true))
  (`/Game/Blueprints/LVL_Artiste3D/BlueprintActor/BP_Button.DeactivateButton` (cast `/Game/Blueprints/LVL_Artiste3D/BlueprintActor/BP_ButtonRGB` (`ChildActorComponent.ChildActor` (`self.BP_ButtonRGB_Increase`)) :!pure true)))

(fn `UserConstructionScript`)