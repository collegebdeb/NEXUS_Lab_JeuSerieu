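; Sliding double door actor that opens on trigger overlap and can lock behind whatever passes through.
; Two timelines slide the panels apart with sound when opening is allowed, and reverse on exit.
; Leaving the inside box away from the door locks it once unless always unlocked, with later exits able to relock it.
; The outside box re-enables opening as softlock prevention; UnlockDoor clears the lock.
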(event `self.TriggerBox.OnComponentBeginOverlap`
  (params (OverlappedComponent :type "PrimitiveComponent Object Reference") (OtherActor :type "Actor Object Reference") (OtherComp :type "PrimitiveComponent Object Reference") (OtherBodyIndex :type Integer) (bFromSweep :type Boolean) (SweepResult :type "HitResult Structure (by ref)"))
  (`self.CanBeOpened`
    (:`then`
      (`GameplayStatics.PlaySound2D` "/Game/SFX/Sliding_Door_CutVersion.Sliding_Door_CutVersion" 1.0 1.0 0.0 null null)
      (`|ExecutionSequence`
        (:`then_0`
          (bind (_direction _door_track) (`Timeline|Open/Close Door` :!label _label)
            (:`Update`
              (`SceneComponent.K2_SetRelativeLocation` (`self.DoorLeft`) (`KismetMathLibrary.MakeVector` (`KismetMathLibrary.Lerp` -125.0 -250.0 _door_track)) false false))))
        (:`then_1`
          (bind (_direction_2 _door_track_2) (`Timeline|Timeline` :!label _label_2)
            (:`Update`
              (`SceneComponent.K2_SetRelativeLocation` (`self.DoorRight`) (`KismetMathLibrary.MakeVector` (`KismetMathLibrary.Lerp` 0.0 150.0 _door_track_2)) false false))))))
    (:`else`)))

(event `self.TriggerBox.OnComponentEndOverlap`
  (params (OverlappedComponent :type "PrimitiveComponent Object Reference") (OtherActor :type "Actor Object Reference") (OtherComp :type "PrimitiveComponent Object Reference") (OtherBodyIndex :type Integer))
  (`GameplayStatics.PlaySound2D` "/Game/SFX/Sliding_Door_CutVersion.Sliding_Door_CutVersion" 1.0 1.0 0.0 null null)
  (`|ExecutionSequence`
    (:`then_0`
      (goto _label :!via `Reverse`))
    (:`then_1`
      (goto _label_2 :!via `Reverse`))))

(event `self.TriggerBoxOutside.OnComponentBeginOverlap`
  (params (OverlappedComponent :type "PrimitiveComponent Object Reference") (OtherActor :type "Actor Object Reference") (OtherComp :type "PrimitiveComponent Object Reference") (OtherBodyIndex :type Integer) (bFromSweep :type Boolean) (SweepResult :type "HitResult Structure (by ref)"))
  ; Softlock Prevention
  (if (== (`KismetArrayLibrary.Array_Find` (`self.GetOverlappingComponents` OtherActor) (`self.TriggerBoxInside`)) -1)
    (set `self.CanBeOpened` true)
    (`KismetSystemLibrary.PrintString` "Anti softlock")))

(event `self.TriggerBoxInside.OnComponentEndOverlap`
  (params (OverlappedComponent :type "PrimitiveComponent Object Reference") (OtherActor :type "Actor Object Reference") (OtherComp :type "PrimitiveComponent Object Reference") (OtherBodyIndex :type Integer))
  (if (and (== (`KismetArrayLibrary.Array_Find` (`self.GetOverlappingComponents` OtherActor) (`self.TriggerBox`)) -1) (not (`self.HasBeenLocked`)))
    (`self.AlwaysUnlocked`
      (:`then`)
      (:`else`
        (`KismetSystemLibrary.PrintString` "lock")
        (set `self.HasBeenLocked` true)
        (set `self.IsLocked` true)
        (set `self.CanBeOpened` false :!label _label_3)))
    (else
      (`self.IsLocked`
        (:`then`
          (`KismetSystemLibrary.PrintString` "relocking")
          (goto _label_3))
        (:`else`
          (`KismetSystemLibrary.PrintString` "you shall pass"))))))

(fn `UnlockDoor`
  (set `self.CanBeOpened` true)
  (set `self.IsLocked` false))

(fn `UserConstructionScript`)