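; Main-room bridge Blueprint that extends when its OnEndOfLine event is called.
; OnEndOfLine starts a near-zero-interval looping timer, capped at once per frame, that drives ExtendBridge.
; Each tick interpolates the current length toward the target at constant speed and applies it as the static mesh's Y scale, clearing the timer once the target is reached.
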(event `self.ReceiveBeginPlay`)

(event `/Game/Blueprints/SystemDialogue/Interfaces/BPI_EventCallAtEndOfLine.OnEndOfLine`
  (bind _returnvalue (`KismetSystemLibrary.K2_SetTimerDelegate` (delegate `ExtendBridge`) 1e-05 true true))
  (set `self.BridgeExtendTimer` _returnvalue))

(event `ExtendBridge`
  (bind _staticmesh (`self.StaticMesh`))
  (bind (_relativescale3d_x _relativescale3d_y _relativescale3d_z) (`KismetMathLibrary.BreakVector` (`SceneComponent.RelativeScale3D` _staticmesh)))
  (bind _returnvalue (`KismetMathLibrary.FInterpTo_Constant` (`self.CurrentBridgeLength`) (`self.TargetBridgeLength`) (`GameplayStatics.GetWorldDeltaSeconds`) (`self.BridgeExtensionSpeed`)))
  (bind _output_get (set `self.CurrentBridgeLength` _returnvalue))
  (`SceneComponent.SetRelativeScale3D` _staticmesh (`KismetMathLibrary.MakeVector` _relativescale3d_x _output_get _relativescale3d_z))
  (if (>= (`self.CurrentBridgeLength`) (`self.TargetBridgeLength`))
    (`KismetSystemLibrary.K2_ClearAndInvalidateTimerHandle` (`self.BridgeExtendTimer`))))

(fn `UserConstructionScript`)